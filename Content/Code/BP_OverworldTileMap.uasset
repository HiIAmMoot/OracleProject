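; Overworld map chunk with four seasonal Paper2D tilemaps, showing one season and blending its edges toward differing neighbours.
; SetSeason moves collision to the chosen tilemap, then CalculateTransition runs on a timer to read adjacent chunks' seasons via TileManagerParent.
; Each other season's matching sides become a transition enum, selecting a mask texture for that layer in the current season's dynamic material.
; Debug text displays coordinates, neighbouring seasons and transitions.
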(event EventBeginPlay
  (bind _tilelocation (Variables|Default|GetTileLocation))
  (bind (_x _y) (Utilities|Struct|BreakIntPoint _tilelocation))
  (Class|PaperTileMapComponent|MakeTileMapEditable (Variables|Default|GetWinterTileMap))
  (Utilities|FlowControl|Delay 0.2)
  (Rendering|Components|TextRender|SetText (Variables|Default|GetCoordinates) (Utilities|Text|ToText(String) (Utilities|String|Append "X: " (Utilities|String|ToString(Integer) _x) " Y: " (Utilities|String|ToString(Integer) _y)))))

(event EventTick
  (params (DeltaSeconds :type Float%20%28single-precision%29)))

(fn ConstructionScript
  (Utilities|FlowControl|Sequence
    (:then_0
      (bind _returnvalue (Rendering|Material|CreateDynamicMaterialInstance "/Game/Assets/Materials/DefaultOverworldMaterial.DefaultOverworldMaterial" "None" :!class /Script/Engine.KismetMaterialLibrary))
      (bind _output_get (Variables|Default|SetSpringMaterialInstance _returnvalue))
      (Rendering|Material|SetMaterial (Variables|Default|GetSpringTileMap) 0 _returnvalue))
    (:then_1
      (bind _returnvalue_2 (Rendering|Material|CreateDynamicMaterialInstance "/Game/Assets/Materials/DefaultOverworldMaterial.DefaultOverworldMaterial" "None" :!class /Script/Engine.KismetMaterialLibrary))
      (Variables|Default|SetSummerMaterialInstance _returnvalue_2)
      (Rendering|Material|SetMaterial (Variables|Default|GetSummerTileMap) 0 _returnvalue_2))
    (:then_2
      (bind _returnvalue_3 (Rendering|Material|CreateDynamicMaterialInstance "/Game/Assets/Materials/DefaultOverworldMaterial.DefaultOverworldMaterial" "None" :!class /Script/Engine.KismetMaterialLibrary))
      (Variables|Default|SetFallMaterialInstance _returnvalue_3)
      (Rendering|Material|SetMaterial (Variables|Default|GetFallTileMap) 0 _returnvalue_3))
    (:then_3
      (bind _returnvalue_4 (Rendering|Material|CreateDynamicMaterialInstance "/Game/Assets/Materials/DefaultOverworldMaterial.DefaultOverworldMaterial" "None" :!class /Script/Engine.KismetMaterialLibrary))
      (Variables|Default|SetWinterMaterialInstance _returnvalue_4)
      (Rendering|Material|SetMaterial (Variables|Default|GetWinterTileMap) 0 _returnvalue_4))
    (:then_4
      (Rendering|SetVisibility (Variables|Default|GetTransitionSeasonRight) (Variables|Default|GetDebug) false))))

(fn SetSeason
  (params (Season :type ESeasons%20Enum :default "NewEnumerator0"))
  (bind _wintertilemap (Variables|Default|GetWinterTileMap))
  (bind _falltilemap (Variables|Default|GetFallTileMap))
  (bind _summertilemap (Variables|Default|GetSummerTileMap))
  (bind _springtilemap (Variables|Default|GetSpringTileMap))
  (Variables|Default|SetCurrentSeason Season)
  (Utilities|FlowControl|Sequence
    (:then_0
      (bind _currenttilemap (Variables|Default|GetCurrentTileMap)
        (:then
          (Collision|SetCollisionEnabled _currenttilemap "NoCollision")
          (Transformation|SetRelativeLocation _currenttilemap "0, 0, 0" false true))
        (:else
          _))
      (switch Utilities|FlowControl|Switch|SwitchonESeasons (Variables|Default|GetCurrentSeason)
        (:NewEnumerator0
          (Collision|SetCollisionEnabled _springtilemap "QueryAndPhysics")
          (Variables|Default|SetCurrentTileMap _springtilemap))
        (:NewEnumerator1
          (Collision|SetCollisionEnabled _summertilemap "QueryAndPhysics")
          (Variables|Default|SetCurrentTileMap _summertilemap))
        (:NewEnumerator2
          (Collision|SetCollisionEnabled _falltilemap "QueryAndPhysics")
          (Variables|Default|SetCurrentTileMap _falltilemap))
        (:NewEnumerator3
          (Collision|SetCollisionEnabled _wintertilemap "QueryAndPhysics")
          (Variables|Default|SetCurrentTileMap _wintertilemap))))
    (:then_1
      (Utilities|Time|SetTimerbyFunctionName 0 "CalculateTransition" 0.5))))

(fn GetCurrentTileMap
  (switch Utilities|FlowControl|Switch|SwitchonESeasons (Variables|Default|GetCurrentSeason)
    (:NewEnumerator0
      (return (Variables|Default|GetSpringTileMap)))
    (:NewEnumerator1
      (return (Variables|Default|GetSummerTileMap)))
    (:NewEnumerator2
      (return (Variables|Default|GetFallTileMap)))
    (:NewEnumerator3
      (return (Variables|Default|GetWinterTileMap)))))

(fn CalculateTransition
  (bind _tilemap (CallFunction|GetCurrentTileMap))
  (bind _tilelocation (Variables|Default|GetTileLocation))
  (bind _tilelocation_2 (Variables|Default|GetTileLocation))
  (bind _tilelocation_3 (Variables|Default|GetTileLocation))
  (bind _firstlayertransitionindex (Variables|Default|GetFirstLayerTransitionIndex))
  (bind _secondlayertransitionindex (Variables|Default|GetSecondLayerTransitionIndex))
  (bind _thirdlayertransitionindex (Variables|Default|GetThirdLayerTransitionIndex))
  (bind _surroundingmapseasons (Variables|Default|GetSurroundingMapSeasons))
  (bind _surroundingmapseasons_2 (Variables|Default|GetSurroundingMapSeasons))
  (bind _surroundingmapseasons_3 (Variables|Default|GetSurroundingMapSeasons))
  (bind _surroundingmapseasons_4 (Variables|Default|GetSurroundingMapSeasons))
  (bind _surroundingmapseasons_5 (Variables|Default|GetSurroundingMapSeasons))
  (bind _tilelocation_4 (Variables|Default|GetTileLocation))
  (bind _firstlayertransitionindex_2 (Variables|Default|GetFirstLayerTransitionIndex))
  (bind _secondlayertransitionindex_2 (Variables|Default|GetSecondLayerTransitionIndex))
  (bind _thirdlayertransitionindex_2 (Variables|Default|GetThirdLayerTransitionIndex))
  (bind _firstlayertransitionindex_3 (Variables|Default|GetFirstLayerTransitionIndex))
  (bind _secondlayertransitionindex_3 (Variables|Default|GetSecondLayerTransitionIndex))
  (bind _thirdlayertransitionindex_3 (Variables|Default|GetThirdLayerTransitionIndex))
  (bind _firstlayertransitionindex_4 (Variables|Default|GetFirstLayerTransitionIndex))
  (bind _secondlayertransitionindex_4 (Variables|Default|GetSecondLayerTransitionIndex))
  (bind _thirdlayertransitionindex_4 (Variables|Default|GetThirdLayerTransitionIndex))
  (bind (_x _y) (Utilities|Struct|BreakIntPoint _tilelocation_4))
  (bind (_x_2 _y_2) (Utilities|Struct|BreakIntPoint _tilelocation))
  (bind (_x_3 _y_3) (Utilities|Struct|BreakIntPoint _tilelocation_3))
  (bind (_x_4 _y_4) (Utilities|Struct|BreakIntPoint _tilelocation_2))
  (Utilities|FlowControl|Sequence
    (:then_0
      ;[1 1 1] Left
      (if (== _x_4 0)
        (Utilities|Map|Add _surroundingmapseasons_3 0 (Variables|Default|GetCurrentSeason))
        (else
          (Utilities|Map|Add _surroundingmapseasons_3 0 (Variables|BP_OverworldTileMap_C|GetCurrentSeason (.TileMap (Default|GetMapTileChunkatLocation (Variables|Default|GetTileManagerParent) (Utilities|Struct|MakeIntPoint (- _x_4 1) _y_4))))))))
    (:then_1
      ;[1 1 1] Right
      (if (== _x_2 (- (Variables|/Game/Code/BP_TileManager.BP_TileManager_C|GetTileMapsAmountY (Variables|Default|GetTileManagerParent)) 1))
        (Utilities|Map|Add _surroundingmapseasons_4 1 (Variables|Default|GetCurrentSeason))
        (else
          (Utilities|Map|Add _surroundingmapseasons_4 1 (Variables|BP_OverworldTileMap_C|GetCurrentSeason (.TileMap (Default|GetMapTileChunkatLocation (Variables|Default|GetTileManagerParent) (Utilities|Struct|MakeIntPoint (+ _x_2 1) _y_2))))))))
    (:then_2
      ;[1 1 1] Top
      (if (== _y_3 0)
        (Utilities|Map|Add _surroundingmapseasons_2 2 (Variables|Default|GetCurrentSeason))
        (else
          (Utilities|Map|Add _surroundingmapseasons_2 2 (Variables|BP_OverworldTileMap_C|GetCurrentSeason (.TileMap (Default|GetMapTileChunkatLocation (Variables|Default|GetTileManagerParent) (Utilities|Struct|MakeIntPoint _x_3 (- _y_3 1)))))))))
    (:then_3
      ;[1 1 1] Bottom
      (if (== _y (- (Variables|/Game/Code/BP_TileManager.BP_TileManager_C|GetTileMapsAmountX (Variables|Default|GetTileManagerParent)) 1))
        (Utilities|Map|Add _surroundingmapseasons_5 3 (Variables|Default|GetCurrentSeason))
        (else
          (Utilities|Map|Add _surroundingmapseasons_5 3 (Variables|BP_OverworldTileMap_C|GetCurrentSeason (.TileMap (Default|GetMapTileChunkatLocation (Variables|Default|GetTileManagerParent) (Utilities|Struct|MakeIntPoint _x (+ _y 1)))))))))
    (:then_4
      (Utilities|FlowControl|Sequence
        (:then_0
          ;[1 1 1] Set Textures
          (Utilities|FlowControl|Sequence
            (:then_0
              (Transformation|SetRelativeLocation _tilemap "0,-6.000000, 0" false true)
              (Rendering|SetVisibility _tilemap true false))
            (:then_1
              (switch Utilities|FlowControl|Switch|SwitchonESeasons (Variables|Default|GetCurrentSeason)
                (:NewEnumerator0
                  (CallFunction|SetTransitionVariables _firstlayertransitionindex_2 "NewEnumerator1")
                  (CallFunction|SetTransitionVariables _secondlayertransitionindex_2 "NewEnumerator2" 1)
                  (CallFunction|SetTransitionVariables _thirdlayertransitionindex_2 "NewEnumerator3" 2)
                  (Rendering|SetVisibility (Variables|Default|GetSummerTileMap) false false)
                  (Rendering|SetVisibility (Variables|Default|GetTransitionSpring) false false)
                  (Rendering|Components|TextRender|SetText (Variables|Default|GetTransitionSummer) (Utilities|Text|ToText(String) (Utilities|String|EnumtoString _firstlayertransitionindex_2)))
                  (Rendering|Components|TextRender|SetText (Variables|Default|GetTransitionFall) (Utilities|Text|ToText(String) (Utilities|String|EnumtoString _secondlayertransitionindex_2)))
                  (Rendering|Components|TextRender|SetText (Variables|Default|GetTransitionWinter) (Utilities|Text|ToText(String) (Utilities|String|EnumtoString _thirdlayertransitionindex_2))))
                (:NewEnumerator1
                  (CallFunction|SetTransitionVariables _firstlayertransitionindex_3 "NewEnumerator2")
                  (CallFunction|SetTransitionVariables _secondlayertransitionindex_3 "NewEnumerator3" 1)
                  (CallFunction|SetTransitionVariables _thirdlayertransitionindex_3 "NewEnumerator0" 2)
                  (Rendering|SetVisibility (Variables|Default|GetFallTileMap) false false)
                  (Rendering|SetVisibility (Variables|Default|GetTransitionSummer) false false)
                  (Rendering|Components|TextRender|SetText (Variables|Default|GetTransitionFall) (Utilities|Text|ToText(String) (Utilities|String|EnumtoString _firstlayertransitionindex_3)))
                  (Rendering|Components|TextRender|SetText (Variables|Default|GetTransitionWinter) (Utilities|Text|ToText(String) (Utilities|String|EnumtoString _secondlayertransitionindex_3)))
                  (Rendering|Components|TextRender|SetText (Variables|Default|GetTransitionSpring) (Utilities|Text|ToText(String) (Utilities|String|EnumtoString _thirdlayertransitionindex_3))))
                (:NewEnumerator2
                  (CallFunction|SetTransitionVariables _firstlayertransitionindex_4 "NewEnumerator3")
                  (CallFunction|SetTransitionVariables _secondlayertransitionindex_4 "NewEnumerator0" 1)
                  (CallFunction|SetTransitionVariables _thirdlayertransitionindex_4 "NewEnumerator1" 2)
                  (Rendering|SetVisibility (Variables|Default|GetWinterTileMap) false false)
                  (Rendering|SetVisibility (Variables|Default|GetTransitionFall) false false)
                  (Rendering|Components|TextRender|SetText (Variables|Default|GetTransitionWinter) (Utilities|Text|ToText(String) (Utilities|String|EnumtoString _firstlayertransitionindex_4)))
                  (Rendering|Components|TextRender|SetText (Variables|Default|GetTransitionSpring) (Utilities|Text|ToText(String) (Utilities|String|EnumtoString _secondlayertransitionindex_4)))
                  (Rendering|Components|TextRender|SetText (Variables|Default|GetTransitionSummer) (Utilities|Text|ToText(String) (Utilities|String|EnumtoString _thirdlayertransitionindex_4))))
                (:NewEnumerator3
                  (CallFunction|SetTransitionVariables _firstlayertransitionindex "NewEnumerator0")
                  (CallFunction|SetTransitionVariables _secondlayertransitionindex "NewEnumerator1" 1)
                  (CallFunction|SetTransitionVariables _thirdlayertransitionindex "NewEnumerator2" 2)
                  (Rendering|SetVisibility (Variables|Default|GetSpringTileMap) false false)
                  (Rendering|SetVisibility (Variables|Default|GetTransitionWinter) false false)
                  (Rendering|Components|TextRender|SetText (Variables|Default|GetTransitionSpring) (Utilities|Text|ToText(String) (Utilities|String|EnumtoString _firstlayertransitionindex)))
                  (Rendering|Components|TextRender|SetText (Variables|Default|GetTransitionSummer) (Utilities|Text|ToText(String) (Utilities|String|EnumtoString _secondlayertransitionindex)))
                  (Rendering|Components|TextRender|SetText (Variables|Default|GetTransitionFall) (Utilities|Text|ToText(String) (Utilities|String|EnumtoString _thirdlayertransitionindex))))))))
        (:then_1
          (bind _keys (Utilities|Map|Keys _surroundingmapseasons))
          (for _array_element _keys
            (switch int _array_element
              (:0
                (Rendering|Components|TextRender|SetText (Variables|Default|GetTransitionSeasonLeft) (Utilities|Text|ToText(String) (Utilities|String|EnumtoString (.Value (Utilities|Map|Find _surroundingmapseasons _array_element))))))
              (:1
                (Rendering|Components|TextRender|SetText (Variables|Default|GetTransitionSeasonRight) (Utilities|Text|ToText(String) (Utilities|String|EnumtoString (.Value (Utilities|Map|Find _surroundingmapseasons _array_element))))))
              (:2
                (Rendering|Components|TextRender|SetText (Variables|Default|GetTransitionSeasonTop) (Utilities|Text|ToText(String) (Utilities|String|EnumtoString (.Value (Utilities|Map|Find _surroundingmapseasons _array_element))))))
              (:3
                (Rendering|Components|TextRender|SetText (Variables|Default|GetTransitionSeasonBottom) (Utilities|Text|ToText(String) (Utilities|String|EnumtoString (.Value (Utilities|Map|Find _surroundingmapseasons _array_element)))))))))))))

(fn GetSeasonMaterialInstance
  (params (Season :type ESeasons%20Enum :default "NewEnumerator0"))
  (switch Utilities|FlowControl|Switch|SwitchonESeasons Season
    (:NewEnumerator0
      (return (Variables|Default|GetSpringMaterialInstance)))
    (:NewEnumerator1
      (return (Variables|Default|GetSummerMaterialInstance)))
    (:NewEnumerator2
      (return (Variables|Default|GetFallMaterialInstance)))
    (:NewEnumerator3
      (return (Variables|Default|GetWinterMaterialInstance)))))

(fn SetTransitionVariables
  (params (TransitionEnum :type ESeasonTransitionDirection%20Enum%20%28by%20ref%29 :default "NewEnumerator16") (SeasonFilter :type ESeasons%20Enum :default "NewEnumerator0") (MaterialIndex :type Integer))
  (bind _surroundingmapseasons (Variables|Default|GetSurroundingMapSeasons))
  (LocalVariables|SetLocalTransition TransitionEnum)
  (bind _keys (Utilities|Map|Keys _surroundingmapseasons))
  (for _array_element _keys
    (if (and (Utilities|Enum|NotEqual(Enum) (.Value (Utilities|Map|Find _surroundingmapseasons _array_element)) (Variables|Default|GetCurrentSeason)) (Utilities|Enum|Equal(Enum) (.Value (Utilities|Map|Find _surroundingmapseasons _array_element)) SeasonFilter))
      (switch int _array_element
        (:0
          (LocalVariables|SetLocalTransition "NewEnumerator2"))
        (:1
          (if (Utilities|Enum|Equal(Enum) (LocalVariables|GetLocalTransition) "NewEnumerator16")
            (LocalVariables|SetLocalTransition "NewEnumerator3")
            (elif (Utilities|Enum|Equal(Enum) (LocalVariables|GetLocalTransition) "NewEnumerator2")
              (LocalVariables|SetLocalTransition "NewEnumerator8"))))
        (:2
          (if (Utilities|Enum|Equal(Enum) (LocalVariables|GetLocalTransition) "NewEnumerator16")
            (LocalVariables|SetLocalTransition "NewEnumerator0")
            (elif (Utilities|Enum|Equal(Enum) (LocalVariables|GetLocalTransition) "NewEnumerator2")
              (LocalVariables|SetLocalTransition "NewEnumerator4")
              (elif (Utilities|Enum|Equal(Enum) (LocalVariables|GetLocalTransition) "NewEnumerator3")
                (LocalVariables|SetLocalTransition "NewEnumerator5")
                (elif (Utilities|Enum|Equal(Enum) (LocalVariables|GetLocalTransition) "NewEnumerator8")
                  (LocalVariables|SetLocalTransition "NewEnumerator11"))))))
        (:3
          (if (Utilities|Enum|Equal(Enum) (LocalVariables|GetLocalTransition) "NewEnumerator16")
            (LocalVariables|SetLocalTransition "NewEnumerator1")
            (elif (Utilities|Enum|Equal(Enum) (LocalVariables|GetLocalTransition) "NewEnumerator2")
              (LocalVariables|SetLocalTransition "NewEnumerator6")
              (elif (Utilities|Enum|Equal(Enum) (LocalVariables|GetLocalTransition) "NewEnumerator3")
                (LocalVariables|SetLocalTransition "NewEnumerator7")
                (elif (Utilities|Enum|Equal(Enum) (LocalVariables|GetLocalTransition) "NewEnumerator8")
                  (LocalVariables|SetLocalTransition "NewEnumerator12")
                  (elif (Utilities|Enum|Equal(Enum) (LocalVariables|GetLocalTransition) "NewEnumerator0")
                    (LocalVariables|SetLocalTransition "NewEnumerator13")
                    (elif (Utilities|Enum|Equal(Enum) (LocalVariables|GetLocalTransition) "NewEnumerator4")
                      (LocalVariables|SetLocalTransition "NewEnumerator9")
                      (elif (Utilities|Enum|Equal(Enum) (LocalVariables|GetLocalTransition) "NewEnumerator5")
                        (LocalVariables|SetLocalTransition "NewEnumerator10")
                        (elif (Utilities|Enum|Equal(Enum) (LocalVariables|GetLocalTransition) "NewEnumerator11")
                          (LocalVariables|SetLocalTransition "NewEnumerator14")))))))))))))
  (|SetBy-RefVar TransitionEnum (LocalVariables|GetLocalTransition))
  (CallFunction|SetSeasonTransitionMaterial (LocalVariables|GetLocalTransition) SeasonFilter MaterialIndex)
  (CallFunction|SetTileMapHeightPriority SeasonFilter (LocalVariables|GetLocalTransition)))

(fn SetSeasonTransitionMaterial
  (params (Transition :type ESeasonTransitionDirection%20Enum :default "NewEnumerator16") (Season :type ESeasons%20Enum :default "NewEnumerator0") (MaterialIndex :type Integer))
  (bind _tilelocation (Variables|Default|GetTileLocation))
  (bind _currentseason (Variables|Default|GetCurrentSeason))
  (bind _materialinstance (CallFunction|GetSeasonMaterialInstance _currentseason))
  (Rendering|Material|SetTextureParameterValue _materialinstance (Utilities|String|StringToName (Utilities|String|Append "TransitionTexture" (Utilities|String|ToString(Integer) MaterialIndex))) (Utilities|Select :Index Transition :NewEnumerator16 "/Engine/EditorLandscapeResources/WhiteSquareTexture.WhiteSquareTexture" :NewEnumerator0 "/Game/Assets/Textures/SeasonTransitionMaps/TileSeasonTransitionUp.TileSeasonTransitionUp" :NewEnumerator1 "/Game/Assets/Textures/SeasonTransitionMaps/TileSeasonTransitionDown.TileSeasonTransitionDown" :NewEnumerator2 "/Game/Assets/Textures/SeasonTransitionMaps/TileSeasonTransitionLeft.TileSeasonTransitionLeft" :NewEnumerator3 "/Game/Assets/Textures/SeasonTransitionMaps/TileSeasonTransitionRight.TileSeasonTransitionRight" :NewEnumerator13 "/Game/Assets/Textures/SeasonTransitionMaps/TileSeasonTransitionUD.TileSeasonTransitionUD" :NewEnumerator8 "/Game/Assets/Textures/SeasonTransitionMaps/TileSeasonTransitionLR.TileSeasonTransitionLR" :NewEnumerator4 "/Game/Assets/Textures/SeasonTransitionMaps/TileSeasonTransitionTopLeft.TileSeasonTransitionTopLeft" :NewEnumerator5 "/Game/Assets/Textures/SeasonTransitionMaps/TileSeasonTransitionTopRight.TileSeasonTransitionTopRight" :NewEnumerator6 "/Game/Assets/Textures/SeasonTransitionMaps/TileSeasonTransitionBottomLeft.TileSeasonTransitionBottomLeft" :NewEnumerator7 "/Game/Assets/Textures/SeasonTransitionMaps/TileSeasonTransitionBottomRight.TileSeasonTransitionBottomRight" :NewEnumerator9 "/Game/Assets/Textures/SeasonTransitionMaps/TileSeasonTransitionLeftUD.TileSeasonTransitionLeftUD" :NewEnumerator10 "/Game/Assets/Textures/SeasonTransitionMaps/TileSeasonTransitionRightUD.TileSeasonTransitionRightUD" :NewEnumerator11 "/Game/Assets/Textures/SeasonTransitionMaps/TileSeasonTransitionTopLR.TileSeasonTransitionTopLR" :NewEnumerator12 "/Game/Assets/Textures/SeasonTransitionMaps/TileSeasonTransitionBottomLR.TileSeasonTransitionBottomLR" :NewEnumerator14 "/Game/Assets/Textures/SeasonTransitionMaps/TileSeasonTransition.TileSeasonTransition"))
  (Rendering|Material|SetScalarParameterValue _materialinstance "LocationX" (Math|Conversions|ToFloat(Integer) (+ (.x _tilelocation) 1)) :!class /Script/Engine.MaterialInstanceDynamic)
  (Rendering|Material|SetScalarParameterValue _materialinstance "LocationY" (Math|Conversions|ToFloat(Integer) (+ (.y _tilelocation) 1)) :!class /Script/Engine.MaterialInstanceDynamic))

(fn SetTileMapHeightPriority
  (params (Season :type ESeasons%20Enum :default "NewEnumerator0") (Transition :type ESeasonTransitionDirection%20Enum :default "NewEnumerator16"))
  (Transformation|SetRelativeLocation (CallFunction|GetTileMap Season) "0, 0, 0" false true))

(fn GetTileMap
  (params (Season :type ESeasons%20Enum :default "NewEnumerator0"))
  (switch Utilities|FlowControl|Switch|SwitchonESeasons Season
    (:NewEnumerator0
      (return (Variables|Default|GetSpringTileMap)))
    (:NewEnumerator1
      (return (Variables|Default|GetSummerTileMap)))
    (:NewEnumerator2
      (return (Variables|Default|GetFallTileMap)))
    (:NewEnumerator3
      (return (Variables|Default|GetWinterTileMap)))))

(fn AddPaperTilemap
  (params (bManualAttachment :type Boolean) (RelativeTransform :type Transform) (NewTileMap :type Paper%20Tile%20Map%20Object%20Reference) (Visibility :type Boolean))
  (bind _returnvalue (AddComponent|AddPaperTileMapComponent bManualAttachment RelativeTransform))
  (Rendering|SetVisibility _returnvalue Visibility false)
  (Class|PaperTileMapComponent|SetTileMap _returnvalue NewTileMap)
  (return _returnvalue))

(fn DestroyPaperTilemap
  (params (Tilemap :type Paper%20Tile%20Map%20Component%20Object%20Reference))
  (Components|DestroyComponent Tilemap))

(fn RebuildCollisionRuntime
  (bind _summertilemap (Variables|Default|GetSummerTileMap))
  (Class|PaperTileMapComponent|RebuildCollision _summertilemap)
  (Transformation|AddWorldOffset _summertilemap "0, 0,-1.000000" false true)
  (Transformation|AddWorldOffset (Variables|Default|GetSpringTileMap) "0, 0,1.000000" false true))