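; Base seed projectile with a box collider, projectile movement, a flat-rotated paper sprite and an empty TriggerSeed event.
; On begin play the box ignores its owner and instigator when moving, then enables collision.
; Each tick fakes height for the sprite by shifting Y by a fraction of actor Z at a fixed render Z, with the FX flipbook following while movement is active.
; Construction applies the configurable gravity scale.
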(event Custom|TriggerSeed
  (params (Actor :type Actor%20Object%20Reference)))

(event EventBeginPlay
  (bind _box (Variables|Default|GetBox))
  (Collision|IgnoreActorwhenMoving _box (Components|GetOwner) true)
  (Collision|IgnoreActorwhenMoving _box (Game|GetInstigator) true)
  (Collision|SetCollisionEnabled (Variables|Default|GetBox) "QueryAndPhysics"))

(event EventTick
  (params (DeltaSeconds :type Float%20%28single-precision%29))
  (bind _returnvalue (Transformation|GetActorLocation))
  (bind (_x _y _z) (Math|Vector|BreakVector _returnvalue))
  (Transformation|SetWorldLocation (Variables|Default|GetPaperSprite) (Math|Vector|MakeVector _x (+ _y (* _z 0.2)) (Variables|Default|GetZLocation)) false true)
  (if (Components|Activation|IsActive (Variables|Default|GetProjectileMovement))
    (bind _seedfxflipbook (Variables|Default|GetSeedFXFlipbook)
      (:then
        (Transformation|SetRelativeLocation _seedfxflipbook (Variables|/Script/Engine.SceneComponent|GetRelativeLocation (Variables|Default|GetPaperSprite)) false true))
      (:else))))

(fn ConstructionScript
  (Variables|/Script/Engine.ProjectileMovementComponent|SetProjectileGravityScale (Variables|Default|GetProjectileMovement) (Variables|Default|GetGravityScale))
  (Transformation|SetWorldRotation (Variables|Default|GetPaperSprite) "0, 0,-90.000000" false false))