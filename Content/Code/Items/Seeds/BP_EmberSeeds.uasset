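; Ember seed projectile that sets fire to burnable BP_BaseInteractable objects.
; The first hit or slightly delayed overlap triggers it once, deactivating movement and collision and swapping the sprite for a fire flipbook.
; A timer then applies heavy damage to any stored burnable target and expires the seed.
; Disconnected leftover nodes include an unused line-trace search for burnable targets.
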(event Custom|DestroyFire
  ;[1 1 1] Apply damage & destroy seed
  (bind _burningactor (Variables|Default|GetBurningActor)
    (:then
      (Game|Damage|ApplyDamage _burningactor 5e+02 (Pawn|GetController (Game|GetInstigator)) (Components|GetOwner)))
    (:else
      _))
  (Actor|SetLifeSpan 0.01))

(event EventBeginPlay
  (|CallParentFunction))

(event Collision|EventActorBeginOverlap
  (params (OtherActor :type Actor%20Object%20Reference))
  ;[1 1 1] Seed triggering
  (Utilities|FlowControl|Delay 0.05) ; Wait a bit before triggering to make the seed overlap a bit with the object
  (CallFunction|TriggerSeed OtherActor))

(event EventTriggerSeed
  (params (Actor :type Actor%20Object%20Reference))
  ;[1 1 1] Trigger seed & play effect
  (Utilities|FlowControl|DoOnce false
    (:Completed
      (Rendering|SetVisibility (Variables|Default|GetPaperSprite) false false)
      (bind _asbp_base_interactable (Utilities|Casting|CastToBP_BaseInteractable Actor)
        (:then
          (if (Variables|/Game/Code/SpecialTiles/BP_BaseInteractable.BP_BaseInteractable_C|GetBurnable _asbp_base_interactable)
            (Variables|Default|SetBurningActor _asbp_base_interactable)
            (Components|Movement|StopMovementImmediately (Variables|Default|GetProjectileMovement))))
        (:CastFailed
          _))
      (Components|Activation|SetActive (Variables|Default|GetProjectileMovement) false false)
      (bind _returnvalue (AddComponent|AddPaperFlipbookComponent false (Transformation|GetRelativeTransform (Variables|Default|GetPaperSprite))))
      (Variables|Default|SetSeedFXFlipbook _returnvalue)
      (Collision|SetCollisionEnabled (Variables|Default|GetBox) "NoCollision")
      (Utilities|Time|SetTimerbyEvent (delegate Custom|DestroyFire) 1.5))))

(event Collision|EventHit
  (params (MyComp :type Primitive%20Component%20Object%20Reference) (Other :type Actor%20Object%20Reference) (OtherComp :type Primitive%20Component%20Object%20Reference) (bSelfMoved :type Boolean) (HitLocation :type Vector :default "0, 0, 0") (HitNormal :type Vector :default "0, 0, 0") (NormalImpulse :type Vector :default "0, 0, 0") (Hit :type Hit%20Result%20Structure%20%28by%20ref%29))
  ;[1 1 1] Seed triggering
  (CallFunction|TriggerSeed Other))

(fn ConstructionScript
  (|CallParentFunction))