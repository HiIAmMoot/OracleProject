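; Tile manager that builds the seasonal overworld at BeginPlay by slicing per-season reference tilemaps into a grid of BP_OverworldTileMap chunk child actors.
; A SeasonTileMap's tile user data sets each chunk's season, and CustomLevelScripts attaches per-chunk LevelScript components.
; Tile user data also drives timer-looped tile animation and spawns Hole and Bush actors on the hero's current chunk.
; Helper functions rewrite individual chunks and rebuild their collision.
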(event Custom|AnimateTiles
  ;[1 1 1] Handle Time Animations
  (bind _values (Utilities|Map|Values (Variables|Default|GetAnimatedTiles)))
  (if (> (Utilities|Array|Length _values) 0)
    (for _array_element _values
      (if (> (Utilities|Array|Length (.TileCoordinates (Utilities|Struct|BreakST_AniTileData _array_element))) 0)
        (for _array_element_2 (.TileCoordinates (Utilities|Struct|BreakST_AniTileData _array_element))
          (Class|PaperTileMapComponent|SetTile (Variables|/Game/Code/BP_OverworldTileMap.BP_OverworldTileMap_C|GetCurrentTileMap (.AsBP%20Overworld%20Tile%20Map (Utilities|Casting|CastToBP_OverworldTileMap (.TileMap (Utilities|Struct|BreakST_AniTileCoords _array_element_2))))) (.X (Utilities|Struct|BreakIntVector (.Coordinates (Utilities|Struct|BreakST_AniTileCoords _array_element_2)))) (.Y (Utilities|Struct|BreakIntVector (.Coordinates (Utilities|Struct|BreakST_AniTileCoords _array_element_2)))) (.Z (Utilities|Struct|BreakIntVector (.Coordinates (Utilities|Struct|BreakST_AniTileCoords _array_element_2)))) (Class|TileMapBlueprintLibrary|MakeTile (Utilities|Array|Get(acopy) (.AnimatedTileIndicies (Utilities|Struct|BreakST_AniTileData _array_element)) (.CurrentAnimatedLoopIndex (Utilities|Struct|BreakST_AniTileData _array_element))) (.TileSet (Class|TileMapBlueprintLibrary|BreakTile (Class|PaperTileMapComponent|GetTile (Variables|/Game/Code/BP_OverworldTileMap.BP_OverworldTileMap_C|GetCurrentTileMap (.AsBP%20Overworld%20Tile%20Map (Utilities|Casting|CastToBP_OverworldTileMap (.TileMap (Utilities|Struct|BreakST_AniTileCoords _array_element_2))))) (.X (Utilities|Struct|BreakIntVector (.Coordinates (Utilities|Struct|BreakST_AniTileCoords _array_element_2)))) (.Y (Utilities|Struct|BreakIntVector (.Coordinates (Utilities|Struct|BreakST_AniTileCoords _array_element_2)))) (.Z (Utilities|Struct|BreakIntVector (.Coordinates (Utilities|Struct|BreakST_AniTileCoords _array_element_2))))))) (.bFlipH (Class|TileMapBlueprintLibrary|BreakTile (Class|PaperTileMapComponent|GetTile (Variables|/Game/Code/BP_OverworldTileMap.BP_OverworldTileMap_C|GetCurrentTileMap (.AsBP%20Overworld%20Tile%20Map (Utilities|Casting|CastToBP_OverworldTileMap (.TileMap (Utilities|Struct|BreakST_AniTileCoords _array_element_2))))) (.X (Utilities|Struct|BreakIntVector (.Coordinates (Utilities|Struct|BreakST_AniTileCoords _array_element_2)))) (.Y (Utilities|Struct|BreakIntVector (.Coordinates (Utilities|Struct|BreakST_AniTileCoords _array_element_2)))) (.Z (Utilities|Struct|BreakIntVector (.Coordinates (Utilities|Struct|BreakST_AniTileCoords _array_element_2))))))) (.bFlipV (Class|TileMapBlueprintLibrary|BreakTile (Class|PaperTileMapComponent|GetTile (Variables|/Game/Code/BP_OverworldTileMap.BP_OverworldTileMap_C|GetCurrentTileMap (.AsBP%20Overworld%20Tile%20Map (Utilities|Casting|CastToBP_OverworldTileMap (.TileMap (Utilities|Struct|BreakST_AniTileCoords _array_element_2))))) (.X (Utilities|Struct|BreakIntVector (.Coordinates (Utilities|Struct|BreakST_AniTileCoords _array_element_2)))) (.Y (Utilities|Struct|BreakIntVector (.Coordinates (Utilities|Struct|BreakST_AniTileCoords _array_element_2)))) (.Z (Utilities|Struct|BreakIntVector (.Coordinates (Utilities|Struct|BreakST_AniTileCoords _array_element_2))))))) (.bFlipD (Class|TileMapBlueprintLibrary|BreakTile (Class|PaperTileMapComponent|GetTile (Variables|/Game/Code/BP_OverworldTileMap.BP_OverworldTileMap_C|GetCurrentTileMap (.AsBP%20Overworld%20Tile%20Map (Utilities|Casting|CastToBP_OverworldTileMap (.TileMap (Utilities|Struct|BreakST_AniTileCoords _array_element_2))))) (.X (Utilities|Struct|BreakIntVector (.Coordinates (Utilities|Struct|BreakST_AniTileCoords _array_element_2)))) (.Y (Utilities|Struct|BreakIntVector (.Coordinates (Utilities|Struct|BreakST_AniTileCoords _array_element_2)))) (.Z (Utilities|Struct|BreakIntVector (.Coordinates (Utilities|Struct|BreakST_AniTileCoords _array_element_2))))))))))
        (Utilities|Map|Add (Variables|Default|GetAnimatedTiles) (.UserDataName (Utilities|Struct|BreakST_AniTileData _array_element)) (Utilities|Struct|MakeST_AniTileData (.TileCoordinates (Utilities|Struct|BreakST_AniTileData _array_element)) (.UserDataName (Utilities|Struct|BreakST_AniTileData _array_element)) (.AnimatedTileIndicies (Utilities|Struct|BreakST_AniTileData _array_element)) (Math|Integer|SelectInt 0 (+ (.CurrentAnimatedLoopIndex (Utilities|Struct|BreakST_AniTileData _array_element)) 1) (>= (.CurrentAnimatedLoopIndex (Utilities|Struct|BreakST_AniTileData _array_element)) (Utilities|Array|LastIndex (.AnimatedTileIndicies (Utilities|Struct|BreakST_AniTileData _array_element))))) (.AnimationInterval (Utilities|Struct|BreakST_AniTileData _array_element)) (.CurrentAnimationTime (Utilities|Struct|BreakST_AniTileData _array_element))))))))

(event EventBeginPlay
  ;[1 1 1] Begin Play
  (Variables|SeasonsTransition|SetShowSeasonSelectionMap false)
  (Rendering|SetVisibility (Variables|Default|GetSeasonTileMap) false false)
  (CallFunction|AppendAnimatedTiles)
  (for (_array_element _array_index) (Variables|Default|GetReferenceTilemap)
    (Actor|SetOwner _array_element self)
    (Class|PaperTileMapComponent|MakeTileMapEditable (Variables|/Script/Paper2D.PaperTileMapActor|GetRenderComponent _array_element))
    (CallFunction|GenerateTileChunks _array_element (Utilities|Enum|ByteToEnumESeasons (Math|Conversions|ToByte(Integer) _array_index))))
  (CallFunction|ApplySeasonstoAllChunks)
  (Utilities|FlowControl|Delay 0.2)
  (bind _values (Utilities|Map|Values (Variables|Default|GetTilemaps)))
  (for _array_element_2 _values
    (Utilities|IsValid _array_element_2
      (:Is%20Valid
        (bind _asbp_overworld_tile_map (Utilities|Casting|CastToBP_OverworldTileMap _array_element_2))
        (CallFunction|UpdateDynamicTiles true false _asbp_overworld_tile_map))))
  (Utilities|FlowControl|Delay 0.1)
  (CallFunction|ClearDynamicTiles)
  (Utilities|FlowControl|Delay 0.2)
  (CallFunction|UpdateLocalDynamicTiles)
  (for _array_element_3 (Variables|Default|GetReferenceTilemap)
    (Actor|DestroyActor _array_element_3)))

(fn ConstructionScript
  (bind _referencetilemap (Variables|Default|GetReferenceTilemap))
  (bind _tilechunksize (Variables|Default|GetTileChunkSize))
  (bind _tilechunksize_2 (Variables|Default|GetTileChunkSize))
  (bind _tilechunksize_3 (Variables|Default|GetTileChunkSize))
  (bind (_x _y) (Math|Vector2D|BreakVector2D _tilechunksize_3))
  (bind _returnvalue (* _tilechunksize_2 8.0))
  (bind _returnvalue_2 (* _tilechunksize 16.0))
  (bind (_x_2 _y_2) (Math|Vector2D|BreakVector2D _returnvalue))
  (bind (_x_3 _y_3) (Math|Vector2D|BreakVector2D _returnvalue_2))
  (Utilities|FlowControl|Sequence
    (:then_0
      ;[1 1 1] Set Season Map
      (for _array_element (Components|GetChildrenComponents (Variables|Default|GetDefaultSceneRoot) false)
        (bind _aspaper_tile_map_component (Utilities|Casting|CastToPaperTileMapComponent _array_element))
        (Variables|Default|SetSeasonTileMap _aspaper_tile_map_component)))
    (:then_1
      ;[1 1 1] Init Tilesize
      (if (> (Utilities|Array|Length _referencetilemap) 0)
        (bind (_mapwidth _mapheight _numlayers) (Class|PaperTileMapComponent|GetMapSize (Variables|/Script/Paper2D.PaperTileMapActor|GetRenderComponent (Utilities|Array|Get(acopy) _referencetilemap))))
        (Variables|Default|SetTileMapsAmountZ _numlayers)
        (bind _output_get (Variables|Default|SetTileMapsAmountX (Math|Float|Ceil (/ (Math|Conversions|ToFloat(Integer) _mapwidth) _x))))
        (bind _output_get_2 (Variables|Default|SetTileMapsAmountY (Math|Float|Ceil (/ (Math|Conversions|ToFloat(Integer) _mapheight) _y))))
        (Transformation|SetRelativeScale3D (Variables|Default|GetPlane) (* (Math|Vector|MakeVector (* _output_get _x_3) (* _output_get_2 _y_3) 1.0) 0.01))
        (Transformation|SetRelativeScale3D (Variables|Default|GetSeasonTileMap) (Math|Vector|MakeVector _x_3 1.0 _y_3))
        (Transformation|SetRelativeLocation (Variables|Default|GetSeasonTileMap) (+ (Math|Vector|MakeVector _x_2 0.0 (* _y_2 -1.0)) "-8.000000, 0,8.000000") false true)
        (Transformation|SetRelativeLocation (Variables|Default|GetPlane) (Math|Vector|MakeVector (.X (Math|Vector|BreakVector (* (Math|Vector|MakeVector (* _output_get _x_3) (* _output_get_2 _y_3) 1.0) 0.5))) 0.0 (* (.Y (Math|Vector|BreakVector (* (Math|Vector|MakeVector (* _output_get _x_3) (* _output_get_2 _y_3) 1.0) 0.5))) -1.0)) false true)))
    (:then_2
      ;[1 1 1] Toggle Season Selection visibility
      (Class|PaperTileMapComponent|MakeTileMapEditable (Variables|Default|GetSeasonTileMap))
      (Class|PaperTileMapComponent|ResizeMap (Variables|Default|GetSeasonTileMap) (Variables|Default|GetTileMapsAmountX) (Variables|Default|GetTileMapsAmountY))
      (Rendering|SetVisibility (Variables|Default|GetSeasonTileMap) (Variables|SeasonsTransition|GetShowSeasonSelectionMap) false))))

(fn GenerateTileChunks
  (params (InTilemap :type Paper%20Tile%20Map%20Actor%20Object%20Reference) (Season :type ESeasons%20Enum :default "NewEnumerator0"))
  (bind _tilechunksize (Variables|Default|GetTileChunkSize))
  (bind _tilechunksize_2 (Variables|Default|GetTileChunkSize))
  (bind (_x _y) (Math|Vector2D|BreakVector2D _tilechunksize))
  (bind (_x_2 _y_2) (Math|Vector2D|BreakVector2D _tilechunksize_2))
  (LocalVariables|SetLocalTileMap InTilemap)
  (for _index (range 0 (- (Variables|Default|GetTileMapsAmountY) 1))
    (for _index_2 (range 0 (- (Variables|Default|GetTileMapsAmountX) 1))
      (LocalVariables|SetTempLoopIndex (Utilities|Struct|MakeIntPoint _index _index_2))
      (switch Utilities|FlowControl|Switch|SwitchonESeasons Season
        (:NewEnumerator0
          (bind _returnvalue (AddComponent|AddChildActorComponent false (Math|Transform|MakeTransform (Class|PaperTileMapComponent|GetTileCenterPosition (Variables|/Script/Paper2D.PaperTileMapActor|GetRenderComponent InTilemap) (* _index (Math|Float|Truncate _x_2)) (* _index_2 (Math|Float|Truncate _y_2)) 0 false))))
          (ChildActorComponent|SetChildActorClass _returnvalue "/Game/Code/BP_OverworldTileMap.BP_OverworldTileMap_C")
          (Utilities|IsValid (Variables|/Script/Engine.ChildActorComponent|GetChildActor _returnvalue)
            (:Is%20Valid
              (bind _asbp_overworld_tile_map (Utilities|Casting|CastToBP_OverworldTileMap (Variables|/Script/Engine.ChildActorComponent|GetChildActor _returnvalue)))
              (if (.ReturnValue (Utilities|Map|Find (Variables|Default|GetCustomLevelScripts) (LocalVariables|GetTempLoopIndex)))
                (if (Utilities|IsValidClass (.Value (Utilities|Map|Find (Variables|Default|GetCustomLevelScripts) (LocalVariables|GetTempLoopIndex))))
                  (bind _returnvalue_2 (Class|OracleStaticLibrary|AddActorComponentfromClass _asbp_overworld_tile_map (.Value (Utilities|Map|Find (Variables|Default|GetCustomLevelScripts) (LocalVariables|GetTempLoopIndex)))))
                  (bind _aslevel_script (Utilities|Casting|CastToLevelScript _returnvalue_2))
                  (Default|SetTilemapParent _aslevel_script _asbp_overworld_tile_map)))
              (LocalVariables|SetLoopingOverWorldTileMap _asbp_overworld_tile_map)
              (Variables|/Game/Code/BP_OverworldTileMap.BP_OverworldTileMap_C|SetTileLocation _asbp_overworld_tile_map (LocalVariables|GetTempLoopIndex))
              (Variables|/Game/Code/BP_OverworldTileMap.BP_OverworldTileMap_C|SetTileManagerParent _asbp_overworld_tile_map self)
              (switch Utilities|FlowControl|Switch|SwitchonESeasons Season :!label _label
                (:NewEnumerator0
                  (LocalVariables|SetLoopingCurrentSeasonTileMap (Variables|/Game/Code/BP_OverworldTileMap.BP_OverworldTileMap_C|GetSpringTileMap (LocalVariables|GetLoopingOverWorldTileMap))))
                (:NewEnumerator1
                  (LocalVariables|SetLoopingCurrentSeasonTileMap (Variables|/Game/Code/BP_OverworldTileMap.BP_OverworldTileMap_C|GetSummerTileMap (LocalVariables|GetLoopingOverWorldTileMap))))
                (:NewEnumerator2
                  (LocalVariables|SetLoopingCurrentSeasonTileMap (Variables|/Game/Code/BP_OverworldTileMap.BP_OverworldTileMap_C|GetFallTileMap (LocalVariables|GetLoopingOverWorldTileMap))))
                (:NewEnumerator3
                  (LocalVariables|SetLoopingCurrentSeasonTileMap (Variables|/Game/Code/BP_OverworldTileMap.BP_OverworldTileMap_C|GetWinterTileMap (LocalVariables|GetLoopingOverWorldTileMap)))))
              (Class|PaperTileMapComponent|MakeTileMapEditable (LocalVariables|GetLoopingCurrentSeasonTileMap))
              (Utilities|FlowControl|Sequence
                (:then_0
                  (switch Utilities|FlowControl|Switch|SwitchonESeasons Season
                    (:NewEnumerator0
                      (Utilities|Map|Add (Variables|Default|GetTilemaps) (LocalVariables|GetTempLoopIndex) (LocalVariables|GetLoopingOverWorldTileMap)))))
                (:then_1
                  (for _index_3 (range 0 (- (Variables|Default|GetTileMapsAmountZ) 1))
                    (for _index_4 (range 0 (- (Math|Float|Truncate _x) 1))
                      (for _index_5 (range 0 (- (Math|Float|Truncate _y) 1))
                        (Class|PaperTileMapComponent|SetTile (LocalVariables|GetLoopingCurrentSeasonTileMap) _index_4 _index_5 _index_3 (Class|PaperTileMapComponent|GetTile (Variables|/Script/Paper2D.PaperTileMapActor|GetRenderComponent (LocalVariables|GetLocalTileMap)) (+ (* _index (Math|Float|Truncate _x_2)) _index_4) (+ _index_5 (* _index_2 (Math|Float|Truncate _y_2))) _index_3)))))
                  (switch Utilities|FlowControl|Switch|SwitchonESeasons Season
                    (:NewEnumerator3
                      (Default|RebuildCollisionRuntime (LocalVariables|GetLoopingOverWorldTileMap))
                      (Default|CallOnTilemapGenerated (LocalVariables|GetLoopingOverWorldTileMap)))))))))
        (:NewEnumerator1
          (if (.ReturnValue (Utilities|Map|Find (Variables|Default|GetTilemaps) (LocalVariables|GetTempLoopIndex))) :!label _label_2
            (Utilities|IsValid (.Value (Utilities|Map|Find (Variables|Default|GetTilemaps) (LocalVariables|GetTempLoopIndex)))
              (:Is%20Valid
                (bind _asbp_overworld_tile_map_2 (Utilities|Casting|CastToBP_OverworldTileMap (.Value (Utilities|Map|Find (Variables|Default|GetTilemaps) (LocalVariables|GetTempLoopIndex)))))
                (LocalVariables|SetLoopingOverWorldTileMap _asbp_overworld_tile_map_2)
                (goto _label)))))
        (:NewEnumerator2
          (goto _label_2))
        (:NewEnumerator3
          (goto _label_2))))))

(fn UpdateDynamicTiles
  (params (UpdateAnimatedTiles :type Boolean) (UpdateDynamicObjects :type Boolean) (OverWorldTileMap :type BP%20Overworld%20Tile%20Map%20Object%20Reference))
  (bind _returnvalue (Class|OracleStaticLibrary|CheckifinEditor))
  (bind _animatedtiles (Variables|Default|GetAnimatedTiles))
  (bind _returnvalue_2 (not _returnvalue))
  (bind _returnvalue_3 (and UpdateAnimatedTiles _returnvalue_2))
  ;[1 1 1] Get Unique Tiles
  (bind _output_get (LocalVariables|SetLocalTileMap OverWorldTileMap))
  (bind _output_get_2 (LocalVariables|SetLocalTileMapComponent (Default|GetCurrentTileMap _output_get)))
  (bind (_mapwidth _mapheight _numlayers) (Class|PaperTileMapComponent|GetMapSize _output_get_2))
  (for _index (range 0 (- _numlayers 1))
    (for _index_2 (range 0 (- _mapwidth 1))
      (for _index_3 (range 0 (- _mapheight 1))
        (Utilities|FlowControl|Sequence
          (:then_0
            (if _returnvalue_3
              ;;[1 1 1] Animated Tiles
              (if (Utilities|String|Contains (Utilities|String|ToString(Name) (Class|TileMapBlueprintLibrary|GetTileUserData (Class|PaperTileMapComponent|GetTile (LocalVariables|GetLocalTileMapComponent) _index_2 _index_3 _index))) "Ani" true)
                (if (.ReturnValue (Utilities|Map|Find _animatedtiles (Utilities|String|ToString(Name) (Class|TileMapBlueprintLibrary|GetTileUserData (Class|PaperTileMapComponent|GetTile (LocalVariables|GetLocalTileMapComponent) _index_2 _index_3 _index)))))
                  (bind _output_get_3 (Variables|Default|SetTempAnimatedTileArray (.TileCoordinates (Utilities|Struct|BreakST_AniTileData (.Value (Utilities|Map|Find _animatedtiles (Utilities|String|ToString(Name) (Class|TileMapBlueprintLibrary|GetTileUserData (Class|PaperTileMapComponent|GetTile (LocalVariables|GetLocalTileMapComponent) _index_2 _index_3 _index)))))))))
                  (Utilities|Array|Add _output_get_3 (Utilities|Struct|MakeST_AniTileCoords (Utilities|Struct|MakeIntVector _index_2 _index_3 _index) (LocalVariables|GetLocalTileMap)))
                  (Utilities|Map|Add _animatedtiles (Utilities|String|ToString(Name) (Class|TileMapBlueprintLibrary|GetTileUserData (Class|PaperTileMapComponent|GetTile (LocalVariables|GetLocalTileMapComponent) _index_2 _index_3 _index))) (Utilities|Struct|MakeST_AniTileData (Variables|Default|GetTempAnimatedTileArray) (.UserDataName (Utilities|Struct|BreakST_AniTileData (.Value (Utilities|Map|Find _animatedtiles (Utilities|String|ToString(Name) (Class|TileMapBlueprintLibrary|GetTileUserData (Class|PaperTileMapComponent|GetTile (LocalVariables|GetLocalTileMapComponent) _index_2 _index_3 _index))))))) (.AnimatedTileIndicies (Utilities|Struct|BreakST_AniTileData (.Value (Utilities|Map|Find _animatedtiles (Utilities|String|ToString(Name) (Class|TileMapBlueprintLibrary|GetTileUserData (Class|PaperTileMapComponent|GetTile (LocalVariables|GetLocalTileMapComponent) _index_2 _index_3 _index))))))) (.CurrentAnimatedLoopIndex (Utilities|Struct|BreakST_AniTileData (.Value (Utilities|Map|Find _animatedtiles (Utilities|String|ToString(Name) (Class|TileMapBlueprintLibrary|GetTileUserData (Class|PaperTileMapComponent|GetTile (LocalVariables|GetLocalTileMapComponent) _index_2 _index_3 _index))))))) (.AnimationInterval (Utilities|Struct|BreakST_AniTileData (.Value (Utilities|Map|Find _animatedtiles (Utilities|String|ToString(Name) (Class|TileMapBlueprintLibrary|GetTileUserData (Class|PaperTileMapComponent|GetTile (LocalVariables|GetLocalTileMapComponent) _index_2 _index_3 _index))))))) (.CurrentAnimationTime (Utilities|Struct|BreakST_AniTileData (.Value (Utilities|Map|Find _animatedtiles (Utilities|String|ToString(Name) (Class|TileMapBlueprintLibrary|GetTileUserData (Class|PaperTileMapComponent|GetTile (LocalVariables|GetLocalTileMapComponent) _index_2 _index_3 _index)))))))))))))
          (:then_1
            (if UpdateDynamicObjects
              ;;[1 1 1] Holes
              (if (Utilities|Enum|Equal(Enum) (Utilities|String|ToString(Name) (Class|TileMapBlueprintLibrary|GetTileUserData (Class|PaperTileMapComponent|GetTile (LocalVariables|GetLocalTileMapComponent) _index_2 _index_3 _index))) "Hole")
                (Utilities|Array|AddUnique (Variables|Default|GetHoleTiles) (Utilities|Struct|MakeIntVector _index_2 _index_3 _index))
                (else
                  ;;[1 1 1] Bushes
                  (if (Utilities|Enum|Equal(Enum) (Utilities|String|ToString(Name) (Class|TileMapBlueprintLibrary|GetTileUserData (Class|PaperTileMapComponent|GetTile (LocalVariables|GetLocalTileMapComponent) _index_2 _index_3 _index))) "Bush")
                    (Utilities|Array|AddUnique (Variables|Default|GetBushTiles) (Utilities|Struct|MakeDynamicObjectStruct (Utilities|Struct|MakeIntVector _index_2 _index_3 _index) (Utilities|String|ToString(Name) (Class|TileMapBlueprintLibrary|GetTileUserData (Class|PaperTileMapComponent|GetTile (LocalVariables|GetLocalTileMapComponent) _index_2 _index_3 _index))))))))))))))
  (Utilities|FlowControl|Sequence
    (:then_0
      (if UpdateDynamicObjects
        (Utilities|FlowControl|Sequence
          (:then_0
            ;[1 1 1] Spawn Holes
            (if (> (Utilities|Array|Length (Variables|Default|GetHoleTiles)) 0)
              (for _array_element (Variables|Default|GetHoleTiles)
                (Game|SpawnActorfromClass "/Game/Code/SpecialTiles/Hole.Hole_C" (Math|Transform|MakeTransform (+ (Transformation|GetWorldLocation (LocalVariables|GetLocalTileMapComponent)) (Math|Vector|MakeVector (* (.X (Utilities|Struct|BreakIntVector _array_element)) 16.0) (* (.Y (Utilities|Struct|BreakIntVector _array_element)) 16.0) (Variables|Default|GetObjectSpawnHeight)))) "AlwaysSpawn" 0 0))))
          (:then_1
            ;[1 1 1] Spawn Bushes
            (if (> (Utilities|Array|Length (Variables|Default|GetBushTiles)) 0)
              (for _array_element_2 (Variables|Default|GetBushTiles)
                (Game|SpawnActorfromClass "/Game/Code/SpecialTiles/Bush.Bush_C" (Math|Transform|MakeTransform (+ (Transformation|GetWorldLocation (LocalVariables|GetLocalTileMapComponent)) (Math|Vector|MakeVector (* (.X (Utilities|Struct|BreakIntVector (.Coordinate (Utilities|Struct|BreakDynamicObjectStruct _array_element_2)))) 16.0) (* (.Y (Utilities|Struct|BreakIntVector (.Coordinate (Utilities|Struct|BreakDynamicObjectStruct _array_element_2)))) 16.0) (Variables|Default|GetObjectSpawnHeight)))) "AlwaysSpawn" 0 (.Coordinate (Utilities|Struct|BreakDynamicObjectStruct _array_element_2)) (LocalVariables|GetLocalTileMapComponent) 0)))))))
    (:then_1
      (if _returnvalue_3
        (if (not (Utilities|Time|IsValidTimerHandle (Variables|Default|GetTileAnimationHandle)))
          ;[1 1 1] Tile Animation
          (bind _returnvalue_4 (Utilities|Time|SetTimerbyFunctionName 0 "AnimateTiles" (Variables|Default|GetAnimatedTilesInterval) true))
          (Variables|Default|SetTileAnimationHandle _returnvalue_4))))))

(fn ClearDynamicTiles
  (Utilities|Array|Clear (Variables|Default|GetHoleTiles))
  (Utilities|Array|Clear (Variables|Default|GetBushTiles))
  (bind _outactors (Actor|GetAllActorsOfClass "/Game/Code/SpecialTiles/Hole.Hole_C"))
  (for _array_element _outactors
    (Actor|DestroyActor _array_element))
  (bind _outactors_2 (Actor|GetAllActorsOfClass "/Game/Code/SpecialTiles/Bush.Bush_C"))
  (for _array_element_2 _outactors_2
    (Actor|DestroyActor _array_element_2)))

(fn UpdateLocalDynamicTiles
  (bind _outactors (Actor|GetAllActorsOfClass "/Game/Code/BP_Hero.BP_Hero_C"))
  (for _array_element _outactors
    (bind _currenttilemap (Variables|/Game/Code/BP_Hero.BP_Hero_C|GetCurrentTilemap _array_element)
      (:then
        (CallFunction|UpdateDynamicTiles false true _currenttilemap))
      (:else))))

(fn ApplySeasonstoAllChunks
  (bind _seasontilemap (Variables|Default|GetSeasonTileMap))
  (bind _keys (Utilities|Map|Keys (Variables|Default|GetTilemaps)))
  (Class|PaperTileMapComponent|GetMapSize _seasontilemap)
  (for _array_element _keys
    (Default|SetSeason (.AsBP%20Overworld%20Tile%20Map (Utilities|Casting|CastToBP_OverworldTileMap (.Value (Utilities|Map|Find (Variables|Default|GetTilemaps) _array_element)))) (Utilities|Enum|ByteToEnumESeasons (Math|Conversions|ToByte(Integer) (Math|Conversions|ToInteger(Byte) (Utilities|String|ToString(Name) (Class|TileMapBlueprintLibrary|GetTileUserData (Class|PaperTileMapComponent|GetTile _seasontilemap (.X (Utilities|Struct|BreakIntPoint _array_element)) (.Y (Utilities|Struct|BreakIntPoint _array_element)))))))))))

(fn GetMapTileChunkatLocation
  (params (Coordinates :type Int%20Point%20Structure))
  (bind _tilemaps (Variables|Default|GetTilemaps))
  (bind (_value _returnvalue) (Utilities|Map|Find _tilemaps Coordinates))
  (if _returnvalue
    (bind _asbp_overworld_tile_map (Utilities|Casting|CastToBP_OverworldTileMap _value)
      (:then
        (return _asbp_overworld_tile_map true))
      (:CastFailed
        _)))
  (return 0 false))

(fn AppendAnimatedTiles
  (bind _animatedtiles2 (Variables|Default|GetAnimatedTiles2))
  (bind _keys (Utilities|Map|Keys _animatedtiles2))
  (for _array_element _keys
    (if (.ReturnValue (Utilities|Map|Find _animatedtiles2 _array_element))
      (Utilities|Map|Add (Variables|Default|GetAnimatedTiles) _array_element (.Value (Utilities|Map|Find _animatedtiles2 _array_element))))))

(fn RegenerateSpecificTileChunks
  (params (UpperLeftCoords :type Int%20Point%20Structure) (BottomRightCoords :type Int%20Point%20Structure) (SpringTileMap :type Paper%20Tile%20Map%20Component%20Object%20Reference) (SummerTileMap :type Paper%20Tile%20Map%20Component%20Object%20Reference) (FallTileMap :type Paper%20Tile%20Map%20Component%20Object%20Reference) (WinterTileMap :type Paper%20Tile%20Map%20Component%20Object%20Reference))
  (bind (_x _y) (Utilities|Struct|BreakIntPoint UpperLeftCoords))
  (bind (_x_2 _y_2) (Utilities|Struct|BreakIntPoint BottomRightCoords))
  (bind _tilechunksize (Variables|Default|GetTileChunkSize))
  (bind _tilechunksize_2 (Variables|Default|GetTileChunkSize))
  (bind (_x_3 _y_3) (Utilities|Struct|BreakIntPoint UpperLeftCoords))
  (bind (_x_4 _y_4) (Math|Vector2D|BreakVector2D _tilechunksize_2))
  (bind (_x_5 _y_5) (Math|Vector2D|BreakVector2D _tilechunksize))
  (LocalVariables|SetTileChunkDimensions (Utilities|Struct|MakeIntPoint (- _x_2 _x) (- _y_2 _y)))
  (for _index (range 0 (.X (Utilities|Struct|BreakIntPoint (LocalVariables|GetTileChunkDimensions))))
    (for _index_2 (range 0 (.Y (Utilities|Struct|BreakIntPoint (LocalVariables|GetTileChunkDimensions))))
      (if (.ReturnValue (Utilities|Map|Find (Variables|Default|GetTilemaps) (Utilities|Struct|MakeIntPoint (+ _x_3 _index) (+ _index_2 _y_3))))
        (bind _asbp_overworld_tile_map (Utilities|Casting|CastToBP_OverworldTileMap (.Value (Utilities|Map|Find (Variables|Default|GetTilemaps) (Utilities|Struct|MakeIntPoint (+ _x_3 _index) (+ _index_2 _y_3))))))
        (Utilities|FlowControl|Sequence
          (:then_0
            (for _index_3 (range 0 (- (Variables|Default|GetTileMapsAmountZ) 1))
              (for _index_4 (range 0 (- (Math|Float|Truncate _x_4) 1))
                (for _index_5 (range 0 (- (Math|Float|Truncate _y_4) 1))
                  (Utilities|FlowControl|Sequence
                    (:then_0
                      (bind _falltilemap (LocalVariables|GetFallTileMap)
                        (:then
                          (Class|PaperTileMapComponent|SetTile (Variables|/Game/Code/BP_OverworldTileMap.BP_OverworldTileMap_C|GetFallTileMap _asbp_overworld_tile_map) _index_4 _index_5 _index_3 (Class|PaperTileMapComponent|GetTile _falltilemap (+ _index_4 (* _index (Math|Float|Truncate _x_5))) (+ _index_5 (* _index_2 (Math|Float|Truncate _y_5))) _index_3)))
                        (:else))))))))
          (:then_1
            (Default|RebuildCollisionRuntime _asbp_overworld_tile_map)))))))

(fn AddCustomScriptComponents
  (bind _customlevelscripts (Variables|Default|GetCustomLevelScripts))
  (bind _keys (Utilities|Map|Keys _customlevelscripts))
  (for _array_element _keys
    (if (.ReturnValue (Utilities|Map|Find _customlevelscripts _array_element))
      (if (Utilities|IsValidClass (.Value (Utilities|Map|Find _customlevelscripts _array_element)))
        (if (.ReturnValue (Utilities|Map|Find (Variables|Default|GetTilemaps) _array_element))
          (bind _asbp_overworld_tile_map (Utilities|Casting|CastToBP_OverworldTileMap (.Value (Utilities|Map|Find (Variables|Default|GetTilemaps) _array_element))))
          (bind _returnvalue (Class|OracleStaticLibrary|AddActorComponentfromClass _asbp_overworld_tile_map (.Value (Utilities|Map|Find _customlevelscripts _array_element))))
          (bind _aslevel_script (Utilities|Casting|CastToLevelScript _returnvalue))
          (Default|SetTilemapParent _aslevel_script _asbp_overworld_tile_map)
          (Default|CallOnTilemapGenerated _asbp_overworld_tile_map))))))

(fn RegenerateSpecificTileChunkfromData
  (params (Coords :type Int%20Point%20Structure) (SpringTileMap :type Array%20of%20Paper%20Tile%20Info%20Structures) (SummerTileMap :type Array%20of%20Paper%20Tile%20Info%20Structures) (FallTileMap :type Array%20of%20Paper%20Tile%20Info%20Structures) (WinterTileMap :type Array%20of%20Paper%20Tile%20Info%20Structures))
  (bind _tilemaps (Variables|Default|GetTilemaps))
  (bind (_value _returnvalue) (Utilities|Map|Find _tilemaps Coords))
  (if _returnvalue
    (bind _asbp_overworld_tile_map (Utilities|Casting|CastToBP_OverworldTileMap _value))
    (Utilities|FlowControl|Sequence
      (:then_0
        (LocalVariables|SetLocalLoopIndex 0)
        (bind (_mapwidth _mapheight _numlayers) (Class|PaperTileMapComponent|GetMapSize (Variables|/Game/Code/BP_OverworldTileMap.BP_OverworldTileMap_C|GetSpringTileMap _asbp_overworld_tile_map)))
        (for _index (range 0 (- _mapwidth 1))
          (for _index_2 (range 0 (- _mapheight 1))
            (for _index_3 (range 0 (- _numlayers 1))
              (Class|PaperTileMapComponent|SetTile (Variables|/Game/Code/BP_OverworldTileMap.BP_OverworldTileMap_C|GetSpringTileMap _asbp_overworld_tile_map) _index _index_2 _index_3 (Utilities|Array|Get(acopy) SpringTileMap (LocalVariables|GetLocalLoopIndex)))
              (Math|Integer|IncrementInt (LocalVariables|GetLocalLoopIndex))))))
      (:then_1
        (LocalVariables|SetLocalLoopIndex 0)
        (bind (_mapwidth_2 _mapheight_2 _numlayers_2) (Class|PaperTileMapComponent|GetMapSize (Variables|/Game/Code/BP_OverworldTileMap.BP_OverworldTileMap_C|GetSummerTileMap _asbp_overworld_tile_map)))
        (for _index_4 (range 0 (- _mapwidth_2 1))
          (for _index_5 (range 0 (- _mapheight_2 1))
            (for _index_6 (range 0 (- _numlayers_2 1))
              (Class|PaperTileMapComponent|SetTile (Variables|/Game/Code/BP_OverworldTileMap.BP_OverworldTileMap_C|GetSummerTileMap _asbp_overworld_tile_map) _index_4 _index_5 _index_6 (Utilities|Array|Get(acopy) SummerTileMap (LocalVariables|GetLocalLoopIndex)))
              (Math|Integer|IncrementInt (LocalVariables|GetLocalLoopIndex))))))
      (:then_2
        (LocalVariables|SetLocalLoopIndex 0)
        (bind (_mapwidth_3 _mapheight_3 _numlayers_3) (Class|PaperTileMapComponent|GetMapSize (Variables|/Game/Code/BP_OverworldTileMap.BP_OverworldTileMap_C|GetFallTileMap _asbp_overworld_tile_map)))
        (for _index_7 (range 0 (- _mapwidth_3 1))
          (for _index_8 (range 0 (- _mapheight_3 1))
            (for _index_9 (range 0 (- _numlayers_3 1))
              (Class|PaperTileMapComponent|SetTile (Variables|/Game/Code/BP_OverworldTileMap.BP_OverworldTileMap_C|GetFallTileMap _asbp_overworld_tile_map) _index_7 _index_8 _index_9 (Utilities|Array|Get(acopy) FallTileMap (LocalVariables|GetLocalLoopIndex)))
              (Math|Integer|IncrementInt (LocalVariables|GetLocalLoopIndex))))))
      (:then_3
        (LocalVariables|SetLocalLoopIndex 0)
        (bind (_mapwidth_4 _mapheight_4 _numlayers_4) (Class|PaperTileMapComponent|GetMapSize (Variables|/Game/Code/BP_OverworldTileMap.BP_OverworldTileMap_C|GetWinterTileMap _asbp_overworld_tile_map)))
        (for _index_10 (range 0 (- _mapwidth_4 1))
          (for _index_11 (range 0 (- _mapheight_4 1))
            (for _index_12 (range 0 (- _numlayers_4 1))
              (Class|PaperTileMapComponent|SetTile (Variables|/Game/Code/BP_OverworldTileMap.BP_OverworldTileMap_C|GetWinterTileMap _asbp_overworld_tile_map) _index_10 _index_11 _index_12 (Utilities|Array|Get(acopy) WinterTileMap (LocalVariables|GetLocalLoopIndex)))
              (Math|Integer|IncrementInt (LocalVariables|GetLocalLoopIndex))))))
      (:then_4
        (Default|RebuildCollisionRuntime _asbp_overworld_tile_map)))))