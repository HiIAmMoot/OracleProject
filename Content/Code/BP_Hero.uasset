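; Player hero for a top-down Paper2D overworld, with four-way movement, RepNotify-driven facing flipbooks and two child-actor item slots on Z and X.
; Tick forward traces report walls and dynamic objects, and trigger timeline cliff jumps from tile user data, landing where downward traces find ground.
; Falling in holes plays a shrink-and-spin, costs health and respawns toward the last valid position.
; Overlapping an overworld tilemap refreshes dynamic tiles.
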(event Custom|SetInHole
  (params (HolePosition :type Vector) (FallInHoleInitialLocation :type Vector) (Instant :type Boolean))
  ;[1 1 1] Fall in Hole
  (if (or (Variables|Default|GetBusy) Instant)
    (Variables|Default|SetInHole true)
    (Variables|Default|SetFallInHoleInitialLocation FallInHoleInitialLocation)
    (CallFunction|FallinHole HolePosition :!label _label)
    (elif (not (Variables|Default|GetInHole))
      (Utilities|FlowControl|Sequence
        (:then_0
          (goto _label_2 Open))
        (:then_1
          (Utilities|FlowControl|Delay 0.3)
          (Utilities|FlowControl|Gate true :!label _label_2
            (:Exit
              (Variables|Default|SetInHole true)
              (Variables|Default|SetFallInHoleInitialLocation FallInHoleInitialLocation)
              (Utilities|FlowControl|RetriggerableDelay 0.6)
              (goto _label))))))))

(event Custom|FallInHole
  (params (HolePosition :type Vector))
  (bind _returnvalue (Transformation|GetActorLocation))
  (bind (_x _y) (Math|Vector|BreakVector HolePosition))
  (bind _sprite (Variables|Default|GetSprite))
  (bind _lastvalidposition (Variables|Default|GetLastValidPosition))
  (bind _sprite_2 (Variables|Default|GetSprite))
  (bind _sprite_3 (Variables|Default|GetSprite))
  (bind _returnvalue_2 (- _lastvalidposition HolePosition))
  (bind _spritecolor (Variables|/Script/Paper2D.PaperFlipbookComponent|GetSpriteColor _sprite))
  (bind _spritecolor_2 (Variables|/Script/Paper2D.PaperFlipbookComponent|GetSpriteColor _sprite_3))
  (bind (_x_2 _y_2) (Math|Vector|BreakVector _returnvalue_2))
  (bind (_r _g _b) (Math|Color|BreakColor _spritecolor))
  (bind (_r_2 _g_2 _b_2) (Math|Color|BreakColor _spritecolor_2))
  (bind _returnvalue_3 (Math|Float|Absolute(Float) _y_2))
  (bind _returnvalue_4 (Math|Float|Absolute(Float) _x_2))
  (bind _returnvalue_5 (== _y_2 0.0))
  (bind _returnvalue_6 (== _x_2 0.0))
  (bind _returnvalue_7 (> _returnvalue_4 _returnvalue_3))
  (bind _returnvalue_8 (/ _y_2 _returnvalue_3))
  (bind _returnvalue_9 (/ _x_2 _returnvalue_4))
  (bind _returnvalue_10 (Math|Float|SelectFloat 1.0 _returnvalue_8 _returnvalue_5))
  (bind _returnvalue_11 (Math|Float|SelectFloat 1.0 _returnvalue_9 _returnvalue_6))
  (bind _returnvalue_12 (Math|Vector|MakeVector 0.0 _returnvalue_10 0.0))
  (bind _returnvalue_13 (Math|Vector|MakeVector _returnvalue_11 0.0 0.0))
  (bind _returnvalue_14 (Math|Vector|SelectVector _returnvalue_13 _returnvalue_12 _returnvalue_7))
  ;[1 1 1] Fall in Hole
  (Utilities|FlowControl|DoOnce false :!label _label
    (:Completed
      (Variables|Default|SetBusy true)
      (Utilities|FlowControl|Sequence
        (:then_0
          (Utilities|FlowControl|Gate true) ; enters at Close
        )
        (:then_1
          (Variables|/Script/Engine.PrimitiveComponent|SetbGenerateOverlapEvents (Variables|Collision|GetCapsuleComponent) false)
          (Variables|Actor|SetbCanBeDamaged false)
          (Utilities|FlowControl|RetriggerableDelay 1.3)
          (bind _index (Utilities|FlowControl|ForLoopwithBreak 1 100 :!label _label_2)
            (:LoopBody
              (bind _outhit (Collision|LineTraceByChannel (+ HolePosition (Math|Vector|MakeVector (.X (Math|Vector|BreakVector (* _returnvalue_14 (* _index 16)))) (.Y (Math|Vector|BreakVector (* _returnvalue_14 (* _index 16)))) (.Z (Math|Vector|BreakVector (Transformation|GetActorLocation))))) (- (+ HolePosition (Math|Vector|MakeVector (.X (Math|Vector|BreakVector (* _returnvalue_14 (* _index 16)))) (.Y (Math|Vector|BreakVector (* _returnvalue_14 (* _index 16)))) (.Z (Math|Vector|BreakVector (Transformation|GetActorLocation))))) "0, 0,100.000000") "TraceTypeQuery1" false 0 "None"))
              (Development|PrintString (Utilities|GetDisplayName (.HitActor (Collision|BreakHitResult _outhit))))
              (Utilities|Casting|CastToStaticMeshActor (.HitActor (Collision|BreakHitResult _outhit)))
              (Transformation|SetActorLocation (Math|Vector|MakeVector (.X (Math|Vector|BreakVector (.ImpactPoint (Collision|BreakHitResult _outhit)))) (.Y (Math|Vector|BreakVector (.ImpactPoint (Collision|BreakHitResult _outhit)))) (.z (Transformation|GetActorLocation))) false true)
              (goto _label_2 Break))
            (:Completed
              (Variables|Default|SetHealth (Math|Integer|Clamp(Integer) (- (Variables|Default|GetHealth) 2) 0 (Variables|Default|GetHealth)))
              (Variables|Default|SetInHole false)
              (CallFunction|BreakFreefromHole)
              (Variables|Actor|SetbCanBeDamaged true)
              (Variables|Default|SetBusy false)
              (CallFunction|ForceSpriteinDirection (* _returnvalue_14 -1))
              (Sprite|SetSpriteColor _sprite_3 (Utilities|Struct|MakeLinearColor _r_2 _g_2 _b_2 1.0))
              (Transformation|SetRelativeScale3D _sprite_3 "1.000000,1.000000,1.000000")
              (Variables|/Script/Engine.PrimitiveComponent|SetbGenerateOverlapEvents (Variables|Collision|GetCapsuleComponent) true)
              (Utilities|FlowControl|Delay 0.2)
              (goto _label Reset))))
        (:then_2
          (Utilities|FlowControl|Delay (Utilities|Time|GetWorldDeltaSeconds))
          (bind _fallspritescale (Timeline|FallInHoleAnimation PlayFromStart)
            (:Update
              (Transformation|SetRelativeRotation _sprite (Math|Rotator|MakeRotator 0.0 (* _fallspritescale 3.6e+02) 0.0) false false)
              (Transformation|SetActorLocation (Math|Vector|Lerp(Vector) (Math|Vector|MakeVector _x (+ _y 1.0) (.Z (Math|Vector|BreakVector _returnvalue))) _returnvalue _fallspritescale) true false)
              (Sprite|SetSpriteColor _sprite (Math|Color|MakeColor _r _g _b _fallspritescale))
              (Sprite|SetFlipbook _sprite_2 (Variables|Default|GetFallHole))
              (Transformation|SetRelativeScale3D _sprite_2 (Math|Conversions|ToVector(Float) _fallspritescale)))))))))

(event Custom|ExecuteCliffJump
  (params (Distance :type Float%20%28single-precision%29) (OriginalLocation :type Vector) (TilesTraveled :type Integer) (JumpDirection :type Vector))
  (bind (_x _y) (Math|Vector|BreakVector OriginalLocation))
  (bind _sprite (Variables|Default|GetSprite))
  (bind _jumpshadow (Variables|Default|GetJumpShadow))
  ;[1 1 1] Jump Off Cliff
  (Utilities|FlowControl|DoOnce false :!label _label
    (:Completed
      (Variables|Default|SetBusy true)
      (Rendering|SetVisibility (Variables|Default|GetJumpShadow) true false)
      (Components|Timeline|SetNewTime (Variables|Default|GetSprite) 0.0)
      (CallFunction|SetJumpAnimation (CallFunction|GetDirectionfromVector JumpDirection))
      (Collision|SetCollisionEnabled (Variables|Collision|GetCapsuleComponent) "NoCollision")
      (Components|Timeline|SetPlayRate (Variables|Default|GetJumpingDown) (CallFunction|GetCliffJumpPlayRate TilesTraveled))
      (bind (_direction _distancetraveled _z_height) (Timeline|JumpingDown PlayFromStart)
        (:Update
          (Transformation|SetActorLocation (+ (Math|Vector|MakeVector _x _y 1e+01) (Math|Vector|MakeVector (.X (Math|Vector|BreakVector (* JumpDirection (* _distancetraveled Distance)))) (.Y (Math|Vector|BreakVector (* JumpDirection (* _distancetraveled Distance)))) (* _z_height 12.0))) false true)
          (Transformation|SetRelativeLocation (Variables|Default|GetSprite) (Math|Vector|MakeVector 0.0 0.0 (+ (* (* _z_height 12.0) 0.9) 1.0)) false true) ; Move Sprite
          (Transformation|SetRelativeLocation _jumpshadow (Math|Vector|MakeVector 0.0 -1.0 (* (* _z_height 12.0) -1.0)) false true)
          (Transformation|SetRelativeScale3D _jumpshadow (Math|Conversions|ToVector(Float) (/ (Math|Float|Clamp(Float) (- 1.0 (Math|Float|Power _z_height 2.0)) 0.01) (- 1.0 (Math|Float|Power _z_height 2.0))))))
        (:Finished
          (Utilities|FlowControl|RetriggerableDelay 0.01)
          (Variables|Default|SetBusy false)
          (Components|Timeline|SetPlayRate _sprite 0.0)
          (Components|Timeline|SetNewTime _sprite 1.0)
          (Collision|SetCollisionEnabled (Variables|Collision|GetCapsuleComponent) "QueryAndPhysics")
          (Rendering|SetVisibility _jumpshadow false false)
          (CallFunction|ForceSpriteinDirection (CallFunction|GetCurrentRotationVector))
          (Utilities|FlowControl|Delay 0.01)
          (goto _label Reset))))))

(event Custom|BreakFreeFromHole
  ;[1 1 1] Fall in Hole
  (Variables|Default|SetInHole false)
  (Variables|Default|SetFallInHoleInitialLocation "0, 0, 0")
  (Utilities|FlowControl|Gate true) ; enters at Close
)

(event EventTick
  (params (DeltaSeconds :type Float%20%28single-precision%29))
  (bind _returnvalue (Transformation|GetActorLocation))
  (bind _outvector (CallFunction|GetCurrentRotationVector))
  (bind _returnvalue_2 (Pawn|GetControlRotation :!class /Script/Engine.Pawn))
  (bind _returnvalue_3 (Input|AxisValues|GetMovingRight))
  (bind _returnvalue_4 (Input|AxisValues|GetMovingDown))
  (bind _secondaryitem (Variables|Default|GetSecondaryItem))
  (bind _primaryitem (Variables|Default|GetPrimaryItem))
  (bind _sprite (Variables|Default|GetSprite))
  (bind _sprite_2 (Variables|Default|GetSprite))
  (bind _returnvalue_5 (Math|Float|Absolute(Float) _returnvalue_4))
  (bind _returnvalue_6 (Math|Float|Absolute(Float) _returnvalue_3))
  (bind _returnvalue_7 (Math|Conversions|RotationFromXVector _outvector))
  (bind _pitch (Math|Rotator|BreakRotator _returnvalue_2))
  (bind _returnvalue_8 (* (.y _returnvalue) 1e+01))
  (bind _returnvalue_9 (* (.x _returnvalue) 1e+01))
  (bind _childactor (Variables|/Script/Engine.ChildActorComponent|GetChildActor _secondaryitem))
  (bind _childactor_2 (Variables|/Script/Engine.ChildActorComponent|GetChildActor _primaryitem))
  (bind _returnvalue_10 (Math|Float|Round _returnvalue_8))
  (bind _returnvalue_11 (Math|Float|Round _returnvalue_9))
  (bind _returnvalue_12 (Math|Rotator|MakeRotator 0.0 _pitch 0.0))
  (bind _returnvalue_13 (Math|Float|Max(Float) _returnvalue_5 _returnvalue_6))
  (bind _returnvalue_14 (Math|Conversions|ToFloat(Integer) _returnvalue_11))
  (bind _returnvalue_15 (Math|Conversions|ToFloat(Integer) _returnvalue_10))
  (bind _returnvalue_16 (* _returnvalue_15 0.1))
  (bind _returnvalue_17 (* _returnvalue_14 0.1))
  (bind _returnvalue_18 (Math|Vector|MakeVector _returnvalue_17 _returnvalue_16 1e+01))
  ;[1 1 1] Sprite Playrate
  (Utilities|FlowControl|Sequence
    (:then_0
      (CallFunction|ForwardTraces (+ (* (Math|Vector|GetRightVector _returnvalue_12) (stale Input|AxisEvents|InputAxisMovingDown AxisValue)) (* (Math|Vector|GetForwardVector _returnvalue_12) (stale Input|AxisEvents|InputAxisMovingRight AxisValue)))))
    (:then_1
      (if (Variables|Default|GetBusy)
        (Components|Timeline|SetPlayRate _sprite 1.0)
        (else
          (Utilities|FlowControl|Sequence
            (:then_0
              ;[1 1 1] Force Z height of 10
              (Transformation|SetActorLocation _returnvalue_18 false true)
              (if (== (Utilities|Array|Length (Collision|GetOverlappingActors "/Game/Code/SpecialTiles/Hole.Hole_C" :!class /Script/Engine.Actor)) 0)
                (Variables|Default|SetLastValidPosition _returnvalue_18)))
            (:then_1
              (if (and (not (> _returnvalue_13 0.2)) (== (Class|PaperFlipbookComponent|GetPlaybackPositioninFrames _sprite) 1))
                (Components|Timeline|SetNewTime _sprite_2 0.0)))
            (:then_2
              (Components|Timeline|SetPlayRate _sprite_2 _returnvalue_13))))))
    (:then_2
      (Development|PrintString (Utilities|String|ToString(Float) (Components|Animation|GetPlayRate _sprite)) true true "(R=0.000000,G=0.660000,B=1.000000,A=1.000000)" DeltaSeconds)
      (Development|PrintString (Utilities|String|ToString(Boolean) (Class|PaperFlipbookComponent|IsLooping _sprite)) true true "(R=0.000000,G=0.660000,B=1.000000,A=1.000000)" DeltaSeconds)
      (Development|PrintString (Utilities|GetDisplayName (Class|PaperFlipbookComponent|GetFlipbook _sprite)) true true "(R=0.000000,G=0.660000,B=1.000000,A=1.000000)" DeltaSeconds))
    (:then_3
      ;[1 1 1] Rotate Held Items
      (Utilities|FlowControl|Sequence
        (:then_0
          (Utilities|IsValid _childactor_2
            (:Is%20Valid
              (Transformation|SetActorRotation _childactor_2 _returnvalue_7))))
        (:then_1
          (Utilities|IsValid _childactor
            (:Is%20Valid
              (Transformation|SetActorRotation _childactor _returnvalue_7))))))))

(event Collision|EventActorBeginOverlap
  (params (OtherActor :type Actor%20Object%20Reference))
  (bind _asbp_overworld_tile_map (Utilities|Casting|CastToBP_OverworldTileMap OtherActor))
  (Variables|Default|SetCurrentTilemap _asbp_overworld_tile_map)
  (bind _outactors (Actor|GetAllActorsOfClass "/Game/Code/BP_DynamicTile.BP_DynamicTile_C"))
  (for _array_element _outactors
    (Default|ClearDynamicTiles _array_element)
    (Default|UpdateLocalDynamicTiles _array_element)))

(event EventBeginPlay
  (bind _self self)
  (bind _self_2 self)
  (bind _primaryitem (Variables|Default|GetPrimaryItem))
  (bind _secondaryitem (Variables|Default|GetSecondaryItem))
  (bind _childactor (Variables|/Script/Engine.ChildActorComponent|GetChildActor _secondaryitem))
  (bind _childactor_2 (Variables|/Script/Engine.ChildActorComponent|GetChildActor _primaryitem))
  ;[1 1 1] Blur Screen
  (ChildActorComponent|SetChildActorClass _primaryitem "/Game/Code/Items/Sword.Sword_C")
  (Actor|SetOwner _childactor_2 _self_2)
  (bind _asbp_item_class (Utilities|Casting|CastToBP_ItemClass _childactor_2))
  (Variables|/Game/Code/Items/BP_ItemClass.BP_ItemClass_C|SetHero _asbp_item_class _self_2)
  (ChildActorComponent|SetChildActorClass _secondaryitem "/Game/Code/Items/RocsFeather.RocsFeather_C")
  (Actor|SetOwner _childactor _self)
  (bind _asbp_item_class_2 (Utilities|Casting|CastToBP_ItemClass _childactor))
  (Variables|/Game/Code/Items/BP_ItemClass.BP_ItemClass_C|SetHero _asbp_item_class_2 _self))

(event Input|AxisEvents|InputAxisMovingRight
  (params (AxisValue :type Float%20%28single-precision%29))
  ;[1 1 1] Horizontal Movement
  (if (not (Variables|Default|GetBusy))
    (Utilities|FlowControl|Sequence
      (:then_0
        (if (not (Variables|Default|GetInHole))
          (Pawn|Input|AddMovementInput (Math|Vector|GetForwardVector (Math|Rotator|MakeRotator 0.0 (.Pitch (Math|Rotator|BreakRotator (Pawn|GetControlRotation :!class /Script/Engine.Pawn))) 0.0)) AxisValue false)))
      (:then_1
        (if (> AxisValue 0.0)
          (if (or (Variables|Default|GetHasSpritePriority) (Variables|Default|GetLockedDirection))
            (if (== (Input|AxisValues|GetMovingDown) 0.0) :!label _label
              (Variables|Default|SetHasSpritePriority false))
            (else
              (Variables|Default|SetHasSpritePriority true)
              (Variables|Default|SetFacingDirection "NewEnumerator3")))
          (elif (< AxisValue 0.0)
            (if (or (Variables|Default|GetHasSpritePriority) (Variables|Default|GetLockedDirection))
              (goto _label)
              (else
                (Variables|Default|SetHasSpritePriority true)
                (Variables|Default|SetFacingDirection "NewEnumerator2")))
            (else
              (goto _label))))))))

(event Input|AxisEvents|InputAxisMovingDown
  (params (AxisValue :type Float%20%28single-precision%29))
  ;[1 1 1] Vertical Movement
  (if (not (Variables|Default|GetBusy))
    (Utilities|FlowControl|Sequence
      (:then_0
        (if (not (Variables|Default|GetInHole))
          (Pawn|Input|AddMovementInput (Math|Vector|GetRightVector (Math|Rotator|MakeRotator 0.0 (.Pitch (Math|Rotator|BreakRotator (Pawn|GetControlRotation :!class /Script/Engine.Pawn))) 0.0)) AxisValue false)))
      (:then_1
        (if (< AxisValue 0.0)
          (if (or (Variables|Default|GetHasSpritePriority) (Variables|Default|GetLockedDirection))
            (if (== (Input|AxisValues|GetMovingRight) 0.0) :!label _label
              (Variables|Default|SetHasSpritePriority false))
            (else
              (Variables|Default|SetHasSpritePriority true)
              (Variables|Default|SetFacingDirection "NewEnumerator1")))
          (elif (> AxisValue 0.0)
            (if (or (Variables|Default|GetHasSpritePriority) (Variables|Default|GetLockedDirection))
              (goto _label)
              (else
                (Variables|Default|SetHasSpritePriority true)
                (Variables|Default|SetFacingDirection "NewEnumerator0")))
            (else
              (goto _label))))))))

(event Input|KeyboardEvents|LeftBracket
  (params (Key :type Key%20Structure))
  (bind _returnvalue (Viewport|GetViewportSize))
  (bind _camera (Variables|Default|GetCamera))
  ;[1 1 1] Camera Zoom
  (:Pressed
    (switch int (Variables|Default|GetZoomIndex)
      (:0
        (Class|CameraComponent|SetOrthoWidth _camera (* (.x _returnvalue) 0.75))
        (Variables|Default|SetZoomIndex 1))
      (:1
        (Class|CameraComponent|SetOrthoWidth _camera (.x _returnvalue))
        (Variables|Default|SetZoomIndex 2))
      (:2
        (Class|CameraComponent|SetOrthoWidth _camera 256.0)
        (Variables|Default|SetZoomIndex 0)))))

(event Input|KeyboardEvents|X
  (params (Key :type Key%20Structure))
  (bind _secondaryitem (Variables|Default|GetSecondaryItem))
  ;[1 1 1] Item Actions
  (:Pressed
    (bind _childactor (Variables|/Script/Engine.ChildActorComponent|GetChildActor _secondaryitem)
      (:then
        (bind _asbp_item_class (Utilities|Casting|CastToBP_ItemClass _childactor))
        (Default|HandleItemPressedServer _asbp_item_class))
      (:else)))
  (:Released
    (bind _childactor_2 (Variables|/Script/Engine.ChildActorComponent|GetChildActor _secondaryitem)
      (:then
        (bind _asbp_item_class_2 (Utilities|Casting|CastToBP_ItemClass _childactor_2))
        (Default|HandleItemReleasedServer _asbp_item_class_2))
      (:else))))

(event Input|KeyboardEvents|Z
  (params (Key :type Key%20Structure))
  (bind _primaryitem (Variables|Default|GetPrimaryItem))
  ;[1 1 1] Item Actions
  (:Pressed
    (bind _childactor (Variables|/Script/Engine.ChildActorComponent|GetChildActor _primaryitem)
      (:then
        (bind _asbp_item_class (Utilities|Casting|CastToBP_ItemClass _childactor))
        (Default|HandleItemPressedServer _asbp_item_class))
      (:else)))
  (:Released
    (Variables|/Script/Engine.ChildActorComponent|GetChildActor _primaryitem
      (:then
        (bind _asbp_item_class_2 (Utilities|Casting|CastToBP_ItemClass _childactor))
        (Default|HandleItemReleasedServer _asbp_item_class_2))
      (:else))))

(fn ConstructionScript)

(fn DetectWall
  (params (Hit :type Hit%20Result%20Structure))
  (bind (_bblockinghit _binitialoverlap _time _distance _location _impactpoint _normal _impactnormal _physmat _hitactor _hitcomponent) (Collision|BreakHitResult Hit))
  (bind _returnvalue (Utilities|Time|GetWorldDeltaSeconds))
  (bind _aspaper_tile_map_component (Utilities|Casting|CastToPaperTileMapComponent _hitcomponent)
    (:then
      (Default|CallOnDetectWall Hit)
      (Development|PrintString (Utilities|String|ToString(Name) (Class|TileMapBlueprintLibrary|GetTileUserData (Class|PaperTileMapComponent|GetTile _aspaper_tile_map_component (Math|Float|Round (* (.X (Math|Vector|BreakVector (- (Transformation|GetWorldLocation _aspaper_tile_map_component) (+ _impactpoint (* _impactnormal -1))))) -0.0625)) (Math|Float|Round (* (.Y (Math|Vector|BreakVector (- (Transformation|GetWorldLocation _aspaper_tile_map_component) (+ _impactpoint (* _impactnormal -1))))) -0.0625)) 1))) true true "(R=0.000000,G=0.660000,B=1.000000,A=1.000000)" _returnvalue)
      (if (Utilities|String|Contains (Utilities|String|ToString(Name) (Class|TileMapBlueprintLibrary|GetTileUserData (Class|PaperTileMapComponent|GetTile _aspaper_tile_map_component (Math|Float|Round (* (.X (Math|Vector|BreakVector (- (Transformation|GetWorldLocation _aspaper_tile_map_component) (+ _impactpoint (* _impactnormal -1))))) -0.0625)) (Math|Float|Round (* (.Y (Math|Vector|BreakVector (- (Transformation|GetWorldLocation _aspaper_tile_map_component) (+ _impactpoint (* _impactnormal -1))))) -0.0625)) 1))) "CliffJump" true)
        (bind _output_get (LocalVariables|SetCliffDirection (Utilities|String|ToString(Name) (Class|TileMapBlueprintLibrary|GetTileUserData (Class|PaperTileMapComponent|GetTile _aspaper_tile_map_component (Math|Float|Round (* (.X (Math|Vector|BreakVector (- (Transformation|GetWorldLocation _aspaper_tile_map_component) (+ _impactpoint (* _impactnormal -1))))) -0.0625)) (Math|Float|Round (* (.Y (Math|Vector|BreakVector (- (Transformation|GetWorldLocation _aspaper_tile_map_component) (+ _impactpoint (* _impactnormal -1))))) -0.0625)) 1)))))
        (switch string _output_get :!label _label
          (:Default
            (LocalVariables|SetJumpDirection "0,1.000000, 0" :!label _label_2))
          (:CliffJumpDown
            (goto _label_2))
          (:CliffJumpUp
            (LocalVariables|SetJumpDirection "0,-1.000000, 0"))
          (:CliffJumpLeft
            (LocalVariables|SetJumpDirection "-1.000000, 0, 0"))
          (:CliffJumpRight
            (LocalVariables|SetJumpDirection "1.000000, 0, 0")))
        (bind _index (Utilities|FlowControl|ForLoopwithBreak 1 20 :!label _label_3)
          (:LoopBody
            (bind _outhit (Collision|LineTraceByChannel (+ (Math|Vector|MakeVector (.X (Math|Vector|BreakVector (+ (Transformation|GetWorldLocation _aspaper_tile_map_component) (Math|Vector|MakeVector (* (Math|Float|Round (* (.X (Math|Vector|BreakVector (- (Transformation|GetWorldLocation _aspaper_tile_map_component) (+ _impactpoint (* _impactnormal -1))))) -0.0625)) 16.0) (* (Math|Float|Round (* (.Y (Math|Vector|BreakVector (- (Transformation|GetWorldLocation _aspaper_tile_map_component) (+ _impactpoint (* _impactnormal -1))))) -0.0625)) 16.0) 0.0)))) (.Y (Math|Vector|BreakVector (+ (Transformation|GetWorldLocation _aspaper_tile_map_component) (Math|Vector|MakeVector (* (Math|Float|Round (* (.X (Math|Vector|BreakVector (- (Transformation|GetWorldLocation _aspaper_tile_map_component) (+ _impactpoint (* _impactnormal -1))))) -0.0625)) 16.0) (* (Math|Float|Round (* (.Y (Math|Vector|BreakVector (- (Transformation|GetWorldLocation _aspaper_tile_map_component) (+ _impactpoint (* _impactnormal -1))))) -0.0625)) 16.0) 0.0)))) (.Z (Math|Vector|BreakVector (Transformation|GetActorLocation)))) (* (LocalVariables|GetJumpDirection) (* _index 16.0))) (- (+ (Math|Vector|MakeVector (.X (Math|Vector|BreakVector (+ (Transformation|GetWorldLocation _aspaper_tile_map_component) (Math|Vector|MakeVector (* (Math|Float|Round (* (.X (Math|Vector|BreakVector (- (Transformation|GetWorldLocation _aspaper_tile_map_component) (+ _impactpoint (* _impactnormal -1))))) -0.0625)) 16.0) (* (Math|Float|Round (* (.Y (Math|Vector|BreakVector (- (Transformation|GetWorldLocation _aspaper_tile_map_component) (+ _impactpoint (* _impactnormal -1))))) -0.0625)) 16.0) 0.0)))) (.Y (Math|Vector|BreakVector (+ (Transformation|GetWorldLocation _aspaper_tile_map_component) (Math|Vector|MakeVector (* (Math|Float|Round (* (.X (Math|Vector|BreakVector (- (Transformation|GetWorldLocation _aspaper_tile_map_component) (+ _impactpoint (* _impactnormal -1))))) -0.0625)) 16.0) (* (Math|Float|Round (* (.Y (Math|Vector|BreakVector (- (Transformation|GetWorldLocation _aspaper_tile_map_component) (+ _impactpoint (* _impactnormal -1))))) -0.0625)) 16.0) 0.0)))) (.Z (Math|Vector|BreakVector (Transformation|GetActorLocation)))) (* (LocalVariables|GetJumpDirection) (* _index 16.0))) "0, 0,100.000000") "TraceTypeQuery1" false 0 "None"))
            (Utilities|Casting|CastToStaticMeshActor (.HitActor (Collision|BreakHitResult _outhit)))
            (goto _label_3 Break))
          (:Completed
            (CallFunction|ExecuteCliffJump (+ (* _index 16.0) 7.0) (Transformation|GetActorLocation) _index (LocalVariables|GetJumpDirection))))
        (else
          (Development|PrintString (Utilities|String|ToString(Name) (Class|TileMapBlueprintLibrary|GetTileUserData (Class|PaperTileMapComponent|GetTile _aspaper_tile_map_component (Math|Float|Round (* (.X (Math|Vector|BreakVector (- (Transformation|GetWorldLocation _aspaper_tile_map_component) (+ _impactpoint (* _impactnormal -1))))) -0.0625)) (Math|Float|Round (* (.Y (Math|Vector|BreakVector (- (Transformation|GetWorldLocation _aspaper_tile_map_component) (+ _impactpoint (* _impactnormal -1))))) -0.0625))))) true true "(R=0.000000,G=0.660000,B=1.000000,A=1.000000)" _returnvalue)
          (if (Utilities|String|Contains (Utilities|String|ToString(Name) (Class|TileMapBlueprintLibrary|GetTileUserData (Class|PaperTileMapComponent|GetTile _aspaper_tile_map_component (Math|Float|Round (* (.X (Math|Vector|BreakVector (- (Transformation|GetWorldLocation _aspaper_tile_map_component) (+ _impactpoint (* _impactnormal -1))))) -0.0625)) (Math|Float|Round (* (.Y (Math|Vector|BreakVector (- (Transformation|GetWorldLocation _aspaper_tile_map_component) (+ _impactpoint (* _impactnormal -1))))) -0.0625))))) "CliffJump" true)
            (LocalVariables|SetCliffDirection (Utilities|String|ToString(Name) (Class|TileMapBlueprintLibrary|GetTileUserData (Class|PaperTileMapComponent|GetTile _aspaper_tile_map_component (Math|Float|Round (* (.X (Math|Vector|BreakVector (- (Transformation|GetWorldLocation _aspaper_tile_map_component) (+ _impactpoint (* _impactnormal -1))))) -0.0625)) (Math|Float|Round (* (.Y (Math|Vector|BreakVector (- (Transformation|GetWorldLocation _aspaper_tile_map_component) (+ _impactpoint (* _impactnormal -1))))) -0.0625))))))
            (goto _label)))))
    (:CastFailed
      (if (Math|Vector|Equal(Vector) (CallFunction|GetCurrentRotationVector) (* _normal -1.0) 0.0001)
        (CallFunction|DetectDynamicObject Hit false)))))

(fn ForceSpriteinDirection
  (params (Direction :type Vector))
  (if (Math|Vector|Equal(Vector) Direction "0.000000,1.000000, 0" 0.0001)
    (Variables|Default|SetFacingDirection "NewEnumerator0")
    (elif (Math|Vector|Equal(Vector) Direction "-1.000000, 0, 0" 0.0001)
      (Variables|Default|SetFacingDirection "NewEnumerator2")
      (elif (Math|Vector|Equal(Vector) Direction "1.000000, 0, 0" 0.0001)
        (Variables|Default|SetFacingDirection "NewEnumerator3")
        (elif (Math|Vector|Equal(Vector) Direction "0.000000,-1.000000, 0" 0.0001)
          (Variables|Default|SetFacingDirection "NewEnumerator1"))))))

(fn GetCliffJumpPlayRate
  (params (Tiles%20Traveled :type Integer))
  (return (Math|Float|SelectFloat (* 3.0 (/ 1.0 (Math|Conversions|ToFloat(Integer) Tiles%20Traveled))) (Math|Float|SelectFloat 1.5 2.0 (== Tiles%20Traveled 1)) (> Tiles%20Traveled 2))))

(fn GetCurrentRotationVector
  (return (Utilities|Select :Index (Variables|Default|GetFacingDirection) :NewEnumerator0 "0,1.000000, 0" :NewEnumerator1 "0.000000,-1.000000, 0" :NewEnumerator2 "-1.000000, 0, 0" :NewEnumerator3 "1.000000, 0, 0")))

(fn OnRepFacingDirection
  (bind _sprite (Variables|Default|GetSprite))
  (bind _sprite_2 (Variables|Default|GetSprite))
  (Default|CallChangeDirection)
  (switch Utilities|FlowControl|Switch|SwitchonECharacterFacingDirection (Variables|Default|GetFacingDirection)
    (:NewEnumerator0
      (Sprite|SetFlipbook _sprite_2 (Variables|Default|GetWalkDown)))
    (:NewEnumerator1
      (Sprite|SetFlipbook _sprite_2 (Variables|Default|GetWalkUp)))
    (:NewEnumerator2
      (Sprite|SetFlipbook _sprite (Variables|Default|GetWalkLeft)))
    (:NewEnumerator3
      (Sprite|SetFlipbook _sprite (Variables|Default|GetWalkRight)))))

(fn ForwardTraces
  (params (ForwardVector :type Vector))
  (bind _outvector (CallFunction|GetCurrentRotationVector))
  (bind _returnvalue (Math|Vector|VectorLength ForwardVector))
  (bind _returnvalue_2 (Transformation|GetActorLocation))
  (bind _primaryitem (Variables|Default|GetPrimaryItem))
  (bind _secondaryitem (Variables|Default|GetSecondaryItem))
  (bind _returnvalue_3 (> _returnvalue 1.0))
  (bind _childactor (Variables|/Script/Engine.ChildActorComponent|GetChildActor _secondaryitem))
  (bind _childactor_2 (Variables|/Script/Engine.ChildActorComponent|GetChildActor _primaryitem))
  (bind _returnvalue_4 (Math|Vector|SelectVector _outvector ForwardVector _returnvalue_3))
  (bind _array (Utilities|Array|MakeArray _childactor_2 _childactor))
  (Variables|Default|SetRealForwardVector ForwardVector)
  (Utilities|FlowControl|Sequence
    (:then_0
      (bind (_outhit _returnvalue_5) (Collision|LineTraceByChannel _returnvalue_2 (+ _returnvalue_2 (* _returnvalue_4 7.0)) "TraceTypeQuery1" false _array "None"))
      (if (and _returnvalue_5 (not (Variables|Default|GetBusy)))
        (CallFunction|DetectWall _outhit)))
    (:then_1
      (bind (_outhit_2 _returnvalue_6) (Collision|SphereTraceByChannel _returnvalue_2 (+ _returnvalue_2 (* _returnvalue_4 1e+01)) 5.0 "TraceTypeQuery1" false _array "None"))
      (if (Math|Boolean|ANDBoolean _returnvalue_6 (not (Variables|Default|GetBusy)) (Math|Vector|Equal(Vector) (CallFunction|GetCurrentRotationVector) (* (.Normal (Collision|BreakHitResult _outhit_2)) -1.0) 0.0001))
        (CallFunction|DetectDynamicObject _outhit_2 true)))))

(fn DetectDynamicObject
  (params (Hit :type Hit%20Result%20Structure) (Far :type Boolean))
  (bind (_bblockinghit _binitialoverlap _time _distance _location _impactpoint _normal _impactnormal _physmat _hitactor _hitcomponent) (Collision|BreakHitResult Hit))
  (if (!= self _hitactor)
    (switch Utilities|FlowControl|Switch|SwitchonECollisionChannel (Collision|GetCollisionObjectType _hitcomponent)
      (:ECC_WorldDynamic
        _)
      (:ECC_Pawn
        _)
      (:ECC_PhysicsBody
        _)
      (:ECC_GameTraceChannel1
        _))
    (Default|CallOnDetectDynamicObject Far Hit)))

(fn SetJumpAnimation
  (params (Direction :type ECharacterFacingDirection%20Enum :default "NewEnumerator0"))
  (if (not (Variables|Default|GetLockedDirection))
    (Sprite|SetFlipbook (Variables|Default|GetSprite) (Utilities|Select :Index Direction :NewEnumerator0 (Variables|Default|GetJumpDown) :NewEnumerator1 (Variables|Default|GetJumpUp) :NewEnumerator2 (Variables|Default|GetJumpLeft) :NewEnumerator3 (Variables|Default|GetJumpRight)))))

(fn GetDirectionfromEnum
  (params (InDirection :type ECharacterFacingDirection%20Enum :default "NewEnumerator0"))
  (return (Utilities|Select :Index InDirection :NewEnumerator0 "0,1.000000, 0" :NewEnumerator1 "0.000000,-1.000000, 0" :NewEnumerator2 "-1.000000, 0, 0" :NewEnumerator3 "1.000000, 0, 0")))

(fn GetDirectionfromVector
  (params (InVector :type Vector))
  (if (Math|Vector|Equal(Vector) InVector "0,1.000000, 0" 0.5)
    (return "NewEnumerator0")
    (elif (Math|Vector|Equal(Vector) InVector "0,-1.000000, 0" 0.5)
      (return "NewEnumerator1")
      (elif (Math|Vector|Equal(Vector) InVector "-1.000000,0.000000, 0" 0.5)
        (return "NewEnumerator2")
        (elif (Math|Vector|Equal(Vector) InVector "1.000000,0.000000, 0" 0.5)
          (return "NewEnumerator3")
          (else
            (return "NewEnumerator0")))))))